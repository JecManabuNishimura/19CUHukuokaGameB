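; Volumetric fog initializer actor that applies a fixed fog setup to the level's Exponential Height Fog.
; Its construction script finds that actor by class and overwrites its component's settings, enabling volumetric fog with dense, fully opaque fog and strongly directional scattering.
; Inscattering, albedo and emissive colors are set to black.
; All work happens at construction; the event graph holds only disabled placeholder events.
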(event EventBeginPlay)

(event Collision|EventActorBeginOverlap
  (params (OtherActor :type Actor%20Object%20Reference)))

(event EventTick
  (params (DeltaSeconds :type Float%20%28single-precision%29)))

(fn ConstructionScript
  (bind _color (Math|Color|MakeColor 0 0 0 255))
  (bind _returnvalue (Actor|GetActorOfClass "/Script/Engine.ExponentialHeightFog"))
  (Class|ExponentialHeightFogComponent|SetFogDensity (Variables|/Script/Engine.ExponentialHeightFog|GetComponent _returnvalue) 1.0)
  (Class|ExponentialHeightFogComponent|SetFogHeightFalloff (Variables|/Script/Engine.ExponentialHeightFog|GetComponent _returnvalue) 0.001)
  (Class|ExponentialHeightFogComponent|SetFogInscatteringColor (Variables|/Script/Engine.ExponentialHeightFog|GetComponent _returnvalue))
  (Class|ExponentialHeightFogComponent|SetFogMaxOpacity (Variables|/Script/Engine.ExponentialHeightFog|GetComponent _returnvalue) 1.0)
  (Class|ExponentialHeightFogComponent|SetStartDistance (Variables|/Script/Engine.ExponentialHeightFog|GetComponent _returnvalue) 0.0)
  (Class|ExponentialHeightFogComponent|SetFogCutoffDistance (Variables|/Script/Engine.ExponentialHeightFog|GetComponent _returnvalue) 0.0)
  (Class|ExponentialHeightFogComponent|SetVolumetricFog (Variables|/Script/Engine.ExponentialHeightFog|GetComponent _returnvalue) true)
  (Class|ExponentialHeightFogComponent|SetVolumetricFogScatteringDistribution (Variables|/Script/Engine.ExponentialHeightFog|GetComponent _returnvalue) 0.9)
  (Class|ExponentialHeightFogComponent|SetVolumetricFogAlbedo (Variables|/Script/Engine.ExponentialHeightFog|GetComponent _returnvalue) _color)
  (Class|ExponentialHeightFogComponent|SetVolumetricFogEmissive (Variables|/Script/Engine.ExponentialHeightFog|GetComponent _returnvalue) (Math|Conversions|ToLinearColor(Color) _color))
  (Class|ExponentialHeightFogComponent|SetVolumetricFogExtinctionScale (Variables|/Script/Engine.ExponentialHeightFog|GetComponent _returnvalue) 3.0)
  (Class|ExponentialHeightFogComponent|SetNonDirectionalInscatteringColorDistance (Variables|/Script/Engine.ExponentialHeightFog|GetComponent _returnvalue) 77777.0))