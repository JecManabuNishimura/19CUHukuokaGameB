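; Fluorescent light fixture Blueprint that flickers continuously at random intervals.
; The construction script creates dynamic material instances for its two tube meshes.
; On Tick, a boolean-guarded cycle dims both materials' MI_FLightPower and toggles the RectLight's visibility, waits briefly, restores brightness and toggles again.
; A longer random delay holds the bright state before the cycle repeats.
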(event EventTick
  (params (DeltaSeconds :type Float%20%28single-precision%29))
  (if (not (Variables|Default|GetbPlayingFLightAnim))
    (Variables|Default|SetbPlayingFLightAnim true)
    (Rendering|Material|SetScalarParameterValue (Variables|Default|GetDynamic%20Material) "MI_FLightPower" 1.0 :!class /Script/Engine.MaterialInstanceDynamic)
    (Rendering|Material|SetScalarParameterValue (Variables|Default|GetDynamic%20Material1) "MI_FLightPower" 1.0 :!class /Script/Engine.MaterialInstanceDynamic)
    (Rendering|ToggleVisibility (Variables|Default|GetRectLight) false)
    (Utilities|FlowControl|Delay (Math|Random|RandomFloatinRange 0.1 1.0))
    (Rendering|Material|SetScalarParameterValue (Variables|Default|GetDynamic%20Material) "MI_FLightPower" 5e+01 :!class /Script/Engine.MaterialInstanceDynamic)
    (Rendering|Material|SetScalarParameterValue (Variables|Default|GetDynamic%20Material1) "MI_FLightPower" 5e+01 :!class /Script/Engine.MaterialInstanceDynamic)
    (Rendering|ToggleVisibility (Variables|Default|GetRectLight) true)
    (Utilities|FlowControl|Delay (Math|Random|RandomFloatinRange 1.0 3.0))
    (Variables|Default|SetbPlayingFLightAnim false)))

(fn ConstructionScript
  (bind _returnvalue (Rendering|Material|CreateDynamicMaterialInstance (Variables|Default|GetStaticMesh) 0 "/Game/Materials/light_material_cylinder.light_material_cylinder" "None" :!class /Script/Engine.PrimitiveComponent))
  (Variables|Default|SetDynamic%20Material _returnvalue)
  (bind _returnvalue_2 (Rendering|Material|CreateDynamicMaterialInstance (Variables|Default|GetStaticMesh1) 0 "/Game/Materials/light_material_cylinder.light_material_cylinder" "None" :!class /Script/Engine.PrimitiveComponent))
  (Variables|Default|SetDynamic%20Material1 _returnvalue_2))