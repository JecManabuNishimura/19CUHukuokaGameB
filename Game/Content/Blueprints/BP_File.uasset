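; BP_File is a file actor that displays left and right page text through a FilePageText widget on its widget component.
; On BeginPlay it caches the widget, binds to the page-turn event dispatcher and fills both pages from inherited getters not defined in this graph.
; Each page turn reruns that text refresh, while Tick copies the current text color to the widget every frame.
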(event Custom|OnFileTrunPageEventDispatcher_イベント_0
  (bind _filepagetextumg (Variables|Default|GetFilePageTextUMG))
  (bind _returnvalue (Class|CanExamineItem|ReturnLeftPageText))
  (Variables|/Game/UI/FilePageText.FilePageText_C|SetTextTempLeft _filepagetextumg (Utilities|Text|ToText(String) _returnvalue))
  (bind _returnvalue_2 (Class|CanExamineItem|ReturnRightPageText))
  (Variables|/Game/UI/FilePageText.FilePageText_C|SetTextTempRight _filepagetextumg (Utilities|Text|ToText(String) _returnvalue_2)))

(event EventBeginPlay
  (bind _asfile_page_text (Utilities|Casting|CastToFilePageText (UserInterface|GetUserWidgetObject (Variables|Default|Getwidget_comp_))))
  (Variables|Default|SetFilePageTextUMG _asfile_page_text)
  (EventDispatchers|AssignOnFileTrunPageEventDispatcher (delegate Custom|OnFileTrunPageEventDispatcher_イベント_0))
  (bind _returnvalue (Class|CanExamineItem|ReturnLeftPageText))
  (Variables|/Game/UI/FilePageText.FilePageText_C|SetTextTempLeft (Variables|Default|GetFilePageTextUMG) (Utilities|Text|ToText(String) _returnvalue))
  (bind _returnvalue_2 (Class|CanExamineItem|ReturnRightPageText))
  (Variables|/Game/UI/FilePageText.FilePageText_C|SetTextTempRight (Variables|Default|GetFilePageTextUMG) (Utilities|Text|ToText(String) _returnvalue_2)))

(event Collision|EventActorBeginOverlap
  (params (OtherActor :type Actor%20Object%20Reference)))

(event EventTick
  (params (DeltaSeconds :type Float%20%28single-precision%29))
  (bind _returnvalue (Class|CanExamineItem|ReturnTextColor))
  (Variables|/Game/UI/FilePageText.FilePageText_C|SetTextColor (Variables|Default|GetFilePageTextUMG) _returnvalue))

(fn ConstructionScript)