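; VR 3D widget actor that shows the command prompt for the item the player is checking, prefixed with the HMD or non-HMD button label.
; BeginPlay fills the text and sizes its background from the string's byte length to fit wide characters.
; Tick scales the widget by camera-to-item distance and eases it toward the player's hit point, offset toward and facing the camera.
; It destroys itself when the item is invalid or no longer checked.
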(event EventBeginPlay
  (bind _asbp_player_character (Utilities|Casting|CastToBP_PlayerCharacter (Game|GetPlayerCharacter 0)))
  (Variables|Default|SetPlayer1 _asbp_player_character)
  (CallFunction|CheckPlayerRef)
  (Utilities|IsValid (Class|PlayerCharacter|ReturnCheckingItem (Variables|Default|GetPlayer1))
    (:Is%20Valid
      (Variables|Default|SetItemIsChecking (Class|PlayerCharacter|ReturnCheckingItem (Variables|Default|GetPlayer1)))
      (bind _asvr_item_command_ui (Utilities|Casting|CastToVR_ItemCommandUI (UserInterface|GetUserWidgetObject (Variables|Default|GetVR_ItemCommandWidget))))
      (Variables|Default|SetVR_Widget _asvr_item_command_ui)
      (if (Class|HeadMountedDisplayFunctionLibrary|IsHeadMountedDisplayEnabled)
        (Utilities|CalandGiveSizeOfBackground (Utilities|String|Append " 右トリガー：" (Class|PlayerCharacter|ReturnCheckingItemCommandName (Variables|Default|GetPlayer1))) (Variables|Default|GetLengthPerWord))
        (Rendering|Components|TextRender|SetText (Variables|/Game/UI/VR_ItemCommandUI.VR_ItemCommandUI_C|GetCommandText (Variables|Default|GetVR_Widget)) (Utilities|Text|ToText(String) (Utilities|String|Append " 右トリガー：" (Class|PlayerCharacter|ReturnCheckingItemCommandName (Variables|Default|GetPlayer1)))))
        (else
          (Utilities|CalandGiveSizeOfBackground (Utilities|String|Append " B：" (Class|PlayerCharacter|ReturnCheckingItemCommandName (Variables|Default|GetPlayer1))) (Variables|Default|GetLengthPerWord))
          (Rendering|Components|TextRender|SetText (Variables|/Game/UI/VR_ItemCommandUI.VR_ItemCommandUI_C|GetCommandText (Variables|Default|GetVR_Widget)) (Utilities|Text|ToText(String) (Utilities|String|Append " B：" (Class|PlayerCharacter|ReturnCheckingItemCommandName (Variables|Default|GetPlayer1)))))))
      (Utilities|IsValid (Variables|Default|GetItemIsChecking)
        (:Is%20Valid
          (Transformation|SetActorLocation (+ (Transformation|GetActorLocation) (* (Math|Vector|Normalize (Math|Vector|GetForwardVector (Utilities|GetRotationfromActortoCamera))) 2e+01)) false false)
          (Transformation|SetActorRotation (Utilities|GetRotationfromActortoCamera)))))))

(event Collision|EventActorBeginOverlap
  (params (OtherActor :type Actor%20Object%20Reference)))

(event EventTick
  (params (DeltaSeconds :type Float%20%28single-precision%29))
  (bind _player1 (Variables|Default|GetPlayer1))
  (bind _itemischecking (Variables|Default|GetItemIsChecking))
  (bind _itemischecking_2 (Variables|Default|GetItemIsChecking))
  (bind _returnvalue (Transformation|GetActorLocation _itemischecking))
  (bind _m_pcamera (Variables|/Script/hukuokaGame.PlayerCharacter|Getm_pCamera _player1))
  (bind _returnvalue_2 (Transformation|GetWorldLocation _m_pcamera))
  (bind _returnvalue_3 (- _returnvalue_2 _returnvalue))
  (bind _returnvalue_4 (Math|Vector|VectorLength _returnvalue_3))
  (bind _returnvalue_5 (/ _returnvalue_4 6e+02))
  (bind _returnvalue_6 (* _returnvalue_5 0.4))
  (Utilities|IsValid (Variables|Default|GetItemIsChecking)
    (:Is%20Valid
      (Transformation|SetWorldScale3D (Variables|Default|GetVR_ItemCommandWidget) (Math|Vector|MakeVector 1.0 _returnvalue_6 _returnvalue_6))
      (Utilities|IsValid _itemischecking_2
        (:Is%20Valid
          (bind _returnvalue_7 (Class|ItemBase|ReturnCheckedState _itemischecking_2))
          (if _returnvalue_7
            (Transformation|SetActorLocation (Math|Interpolation|VInterpTo (Transformation|GetActorLocation) (+ (Variables|/Script/hukuokaGame.PlayerCharacter|Getvr_ItemHitPoint (Variables|Default|GetPlayer1)) (* (Math|Vector|Normalize (Math|Vector|GetForwardVector (Utilities|GetRotationfromActortoCamera))) 2e+01)) DeltaSeconds 1e+01) false false)
            (Transformation|SetActorRotation (Math|Interpolation|RInterpTo (Transformation|GetActorRotation) (Utilities|GetRotationfromActortoCamera) DeltaSeconds 15.0))
            (else
              (Actor|DestroyActor :!label _label))))
        (:Is%20Not%20Valid
          (goto _label))))
    (:Is%20Not%20Valid
      (goto _label))))

(fn ConstructionScript)

(fn CheckPlayerRef
  (bind _returnvalue (Game|GetPlayerCharacter 0))
  (if (Utilities|IsValid (Variables|Default|GetPlayer1))
    (return)
    (elif (Utilities|IsValid _returnvalue)
      (bind _asbp_player_character (Utilities|Casting|CastToBP_PlayerCharacter _returnvalue)
        (:then
          (Variables|Default|SetPlayer1 _asbp_player_character)
          (if (Utilities|IsValid (Variables|Default|GetPlayer1))
            (return)
            (else
              (Development|PrintString "Failed To Acess  BP_PlayerCharacter" true true "(R=1.000000,G=0.000000,B=0.109215,A=1.000000)" 5.0))))
        (:CastFailed
          (Development|PrintString "Cast Failed of BP_PlayerCharacter" true true "(R=1.000000,G=0.000000,B=0.109215,A=1.000000)" 5.0)))
      (else
        (Development|PrintString "Can't Get Player in VRSmartPhone" true true "(R=1.000000,G=0.000000,B=0.109215,A=1.000000)" 5.0)))))