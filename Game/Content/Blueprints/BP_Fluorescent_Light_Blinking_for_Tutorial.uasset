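; Flickering fluorescent tube light for the tutorial, held until BP_TutorialGameMode's CanLightOn flag, polled every second, lets its power-on timeline play.
; When that finishes, FlashingType picks one of two blink timeline macros, started at a random time offset and playing positional sounds; a third is unwired.
; The timelines drive Intensity into both the RectLight and a dynamic material shared by two meshes, keeping glow and lighting in sync.
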(event EventBeginPlay
  (|SetDMI)
  (Utilities|FlowControl|Sequence
    (:then_0
      (bind _新規track_0 (Timeline|タイムライン_1 PlayFromStart)
        (:Update
          (Variables|Default|Setintensity _新規track_0)
          (Rendering|Material|SetScalarParameterValue (Variables|Default|GetDynamic%20Material) "MI_FLightPower" (Variables|Default|Getintensity) :!class /Script/Engine.MaterialInstanceDynamic)
          (Rendering|Components|Light|SetIntensity (Variables|Default|GetRectLight) (Variables|Default|Getintensity)))
        (:Finished
          (switch int (Variables|Default|GetFlashing_Type)
            (:Default
              (|Blinking0 :!label _label
                (:Update
                  _)))
            (:0
              (goto _label))
            (:1
              (|Blinking1
                (:Update
                  _))))
          (Rendering|Material|SetScalarParameterValue (Variables|Default|GetDynamic%20Material) "MI_FLightPower" (Variables|Default|Getintensity) :!class /Script/Engine.MaterialInstanceDynamic)
          (Rendering|Components|Light|SetIntensity (Variables|Default|GetRectLight) (* (Variables|Default|Getintensity) 1.25)))))
    (:then_1
      (Timeline|タイムライン_1 Stop))
    (:then_2
      (bind _asbp_tutorial_game_mode (Utilities|Casting|CastToBP_TutorialGameMode (Game|GetGameMode)))
      (if (Variables|/Game/Blueprints/BP_TutorialGameMode.BP_TutorialGameMode_C|GetcanLightOn _asbp_tutorial_game_mode) :!label _label_2
        (Timeline|タイムライン_1 Play)
        (else
          (Utilities|FlowControl|Delay 1.0)
          (goto _label_2))))))

(event EventTick
  (params (DeltaSeconds :type Float%20%28single-precision%29)))

(fn ConstructionScript)