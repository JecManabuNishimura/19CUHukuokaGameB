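; Player character Blueprint that handles crouching in PC and VR modes, an item command widget and smartphone damage state.
; On PC a FlipFlop input toggles crouch, while in VR Tick crouches when headset height drops to 70% of a standing height recorded by the ResetHeight input.
; Item check dispatchers add or remove the ItemCommand widget from the viewport.
; SetSmartPhoneDamaged switches the VR smartphone between damaged and reset.
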(event Custom|OnItemCheckBeginEventDispatcher_0
  (UserInterface|Viewport|AddtoViewport (Variables|Default|GetitemCommand) 0))

(event Custom|OnItemCheckEndEventDispatcher_0
  (Widget|RemovefromParent (Variables|Default|GetitemCommand)))

(event EventBeginPlay
  (bind _returnvalue (UserInterface|CreateWidget "/Game/UI/ItemCommand.ItemCommand_C"))
  (Variables|Default|SetitemCommand _returnvalue)
  (EventDispatchers|AssignOnItemCheckBeginEventDispatcher (delegate Custom|OnItemCheckBeginEventDispatcher_0))
  (EventDispatchers|AssignOnItemCheckEndEventDispatcher (delegate Custom|OnItemCheckEndEventDispatcher_0))
  ;[1 1 1] しゃがむの時最大の移動速度
  (Variables|/Script/Engine.CharacterMovementComponent|SetMaxWalkSpeedCrouched (Variables|Character|GetCharacterMovement) (Variables|Default|Getm_MaxWalkSpeed_Crouch)))

(event Collision|EventActorBeginOverlap
  (params (OtherActor :type Actor%20Object%20Reference)))

(event EventTick
  (params (DeltaSeconds :type Float%20%28single-precision%29))
  ;[1 1 1] VRモードなのか？
  (if (Class|HeadMountedDisplayFunctionLibrary|IsHeadMountedDisplayEnabled)
    (Variables|Default|Setvr_isVRmode true)
    ;[1 1 1] VRモードの時しゃがむの判定
    (if (<= (.z (.DevicePosition (Class|HeadMountedDisplayFunctionLibrary|GetOrientationandPosition))) (* (Variables|Default|Getm_VRPlayersHeight) 0.7))
      (Character|Crouch)
      (Variables|Default|Setm_isStanding false)
      (else
        (Character|UnCrouch)
        (Variables|Default|Setm_isStanding true)))
    (else
      (Variables|Default|Setvr_isVRmode false))))

(event EventOnEndCrouch
  (params (HalfHeightAdjust :type Float%20%28single-precision%29) (ScaledHalfHeightAdjust :type Float%20%28single-precision%29))
  ;[1 1 1] PCモード　しゃがむの処理
  (Variables|Default|Setm_isStanding true))

(event EventSetSmartPhoneDamaged
  (params (_value :type Boolean))
  (bind _asbp_vrsmart_phone (Utilities|Casting|CastToBP_VRSmartPhone (Variables|Default|Getvr_Phone)))
  (if _value
    (Default|Damaged _asbp_vrsmart_phone)
    (else
      (Default|Reset _asbp_vrsmart_phone))))

(event Input|ActionEvents|InputActionResetHeight
  (params (Key :type Key%20Structure :default "None"))
  ;[1 1 1] VRモードの時、プレイヤー立っているの高さを設定
  (:Pressed
    (if (Variables|Default|Getvr_isVRmode)
      (Variables|Default|Setm_VRPlayersHeight (.z (.DevicePosition (Class|HeadMountedDisplayFunctionLibrary|GetOrientationandPosition)))))))

(event Input|ActionEvents|InputActionPlayerSquat
  (params (Key :type Key%20Structure :default "None"))
  ;[1 1 1] PCモード　しゃがむの処理
  (:Pressed
    (Utilities|FlowControl|FlipFlop
      (:A
        (Character|Crouch)
        (Variables|Default|Setm_isStanding false))
      (:B
        (Character|UnCrouch)
        (Variables|Default|Setm_isStanding true)))))

(fn ConstructionScript)