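; Player character Blueprint supporting both PC and VR play, with adjustable movement speed and an item-check widget.
; PC crouch moves the spring arm with temporary camera lag, while VR crouch follows headset height against a resettable standing height.
; In VR, Tick box-overlaps at the camera to black out the view inside non-exempt meshes.
; Damage events forward to the VR smartphone, and a fade event opens the GameOver level.
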(event Custom|OnItemCheckBeginEventDispatcher_0
  ;[1 1 1] アイテムコマンドUIをビューポートに追加
  (UserInterface|Viewport|AddtoViewport (Variables|Default|GetitemCommand) 0))

(event Custom|OnItemCheckEndEventDispatcher_0
  ;[1 1 1] (アイテムコマンドUIをビューポートから削除
  (Widget|RemovefromParent (Variables|Default|GetitemCommand)))

(event EventBeginPlay
  ;[1 1 1] BeginPlay
  (bind _returnvalue (UserInterface|CreateWidget "/Game/UI/ItemCommand.ItemCommand_C"))
  (Variables|Default|SetitemCommand _returnvalue)
  (EventDispatchers|AssignOnItemCheckBeginEventDispatcher (delegate Custom|OnItemCheckBeginEventDispatcher_0))
  (EventDispatchers|AssignOnItemCheckEndEventDispatcher (delegate Custom|OnItemCheckEndEventDispatcher_0))
  ;[1 1 1] しゃがむの時最大の移動速度
  (Variables|/Script/Engine.CharacterMovementComponent|SetMaxWalkSpeedCrouched (Variables|Character|GetCharacterMovement) (Variables|Default|GetCrouchSpeed_PC))
  (if (Class|HeadMountedDisplayFunctionLibrary|IsHeadMountedDisplayEnabled)
    ;[1 1 1] Player's Height
    (Utilities|SetPlayerCameraHeight 0.0)
    (else
      (Utilities|SetPlayerCameraHeight (Variables|Default|GetPlayerHeight)
        (:execOut
          (Transformation|SetRelativeLocation (Variables|Default|Getm_pCameraBase) "0, 0,-20.000000" false false))))))

(event Collision|EventActorBeginOverlap
  (params (OtherActor :type Actor%20Object%20Reference)))

(event EventHandDamaged
  ;[1 1 1] ダメージ状態の処理（BP側）
  (bind _asbp_vrsmart_phone (Utilities|Casting|CastToBP_VRSmartPhone (Variables|Default|Getvr_Phone)))
  (Default|HandDamged _asbp_vrsmart_phone))

(event EventEarDamaged
  ;[1 1 1] ダメージ状態の処理（BP側）
  (bind _asbp_vrsmart_phone (Utilities|Casting|CastToBP_VRSmartPhone (Variables|Default|Getvr_Phone)))
  (Default|EarDamaged _asbp_vrsmart_phone))

(event EventTick
  (params (DeltaSeconds :type Float%20%28single-precision%29))
  (bind _self self)
  ;[1 1 1] Tick
  ;[1 1 1] VRモードなのか？
  (if (Class|HeadMountedDisplayFunctionLibrary|IsHeadMountedDisplayEnabled)
    (Utilities|FlowControl|Sequence
      (:then_0
        ;[1 1 1] VR Check if HMD needs to black out
        (bind _returnbool (CallFunction|CheckCameratoPlayerDistance (Variables|Default|GetVR_HMD_MaxRnage)))
        (if _returnbool
          _
          (else
            _))
        (bind (_outcomponents _returnvalue) (Collision|BoxOverlapComponents (+ (Transformation|GetWorldLocation (Variables|Default|Getm_pCamera)) (* (Math|Vector|GetForwardVector (Variables|Default|Getm_pCamera)) -1.0)) "15.000000,20.000000,15.000000" (Utilities|Array|MakeArray "ObjectTypeQuery1" "ObjectTypeQuery2") "/Script/Engine.StaticMeshComponent" (Utilities|Array|MakeArray _self (Variables|Default|Getvr_Phone _self) (Variables|Default|GetLeftController _self) (Variables|Default|GetRightController _self)) :!class /Script/Engine.KismetSystemLibrary))
        (if _returnvalue
          (if (> (Utilities|Array|Length _outcomponents) 0)
            (for _array_element _outcomponents
              (if (not (Math|Boolean|ORBoolean (Utilities|ClassIsChildOf (Utilities|GetClass (Components|GetOwner _array_element)) 0) (Utilities|ClassIsChildOf (Utilities|GetClass (Components|GetOwner _array_element)) "/Game/Blueprints/BP_AutomaticDoorLever.BP_AutomaticDoorLever_C") (Utilities|ClassIsChildOf (Utilities|GetClass (Components|GetOwner _array_element)) "/Game/Blueprints/BP_CardKey.BP_CardKey_C")))
                (if (not (Actor|ActorHasTag (Components|GetOwner _array_element) "VR_HMD_BlackoutIgnore"))
                  (Variables|Default|SetisOutOfRange true))))
            (if (Variables|Default|GetisOutOfRange)
              (if (not (Variables|Default|GetisBlackOut))
                (Variables|Default|SetisBlackOut true)
                (CameraFades|StartCameraFade :self (Game|GetPlayerCameraManager 0) :FromAlpha 1.0 :ToAlpha 1.0 :Duration 0.01 :bHoldWhenFinished true))))
          (elif (Variables|Default|GetisBlackOut)
            (CameraFades|StartCameraFade :self (Game|GetPlayerCameraManager 0) :FromAlpha 1.0 :Duration 0.3)
            (Variables|Default|SetisBlackOut false)
            (Variables|Default|SetisOutOfRange false))))
      (:then_1
        (Variables|Default|Setvr_isVRmode true)
        ;[1 1 1] VRモードの時しゃがむの判定
        (if (<= (.z (.DevicePosition (Class|HeadMountedDisplayFunctionLibrary|GetOrientationandPosition))) (* (Variables|Default|Getm_VRPlayersHeight) 0.6))
          (Character|Crouch)
          (Variables|Default|Setm_isStanding false)
          (Transformation|SetRelativeLocation (Variables|Default|Getm_pCameraBase) (Math|Vector|MakeVector 0.0 0.0 (Variables|Default|GetVR_Crouch_Height)) false false)
          (else
            (Character|UnCrouch)
            (Variables|Default|Setm_isStanding true)
            (Transformation|SetRelativeLocation (Variables|Default|Getm_pCameraBase) (Math|Vector|MakeVector 0.0 0.0 (Variables|Default|GetVR_Players_Height)) false false)))))
    (else
      (Variables|Default|Setvr_isVRmode false)
      ;[1 1 1] PCモード 物の下に隠れてから外に出ていくの時、カメラ視線を調整
      (if (Variables|Default|Getm_isCrouch_PC)
        (if (not (Variables|Default|GetbIsCrouched))
          (if (not (AI|Components|NavMovement|IsCrouching (Variables|Character|GetCharacterMovement)))
            (Variables|/Script/Engine.SpringArmComponent|SetbEnableCameraLag (Variables|Default|Getm_pSpringArm) true)
            (Variables|Default|Setm_isStanding true)
            (Variables|Default|Setm_isCrouch_PC false)
            (Utilities|SetPlayerCameraHeight (Variables|Default|GetPlayerHeight)
              (:execOut
                (Utilities|FlowControl|Delay (Variables|Default|GetCrouchCoolTime_PC))
                (Variables|/Script/Engine.SpringArmComponent|SetbEnableCameraLag (Variables|Default|Getm_pSpringArm) false)))))))))

(event EventFadeDameged
  (bind _outactors (Actor|GetAllActorsOfClass "/Game/Blueprints/BP_VRSmartPhone.BP_VRSmartPhone_C"))
  (bind _output_get (Variables|Default|SetSmartPhone _outactors))
  ;[1 1 1] ダメージ状態の処理（BP側）
  (Input|DisableInput _output_get (Game|GetPlayerController 0))
  (bind _returnvalue (UserInterface|CreateWidget "/Game/UI/Fadein_Black.Fadein_Black_C"))
  (UserInterface|Viewport|AddtoViewport _returnvalue 0)
  (Utilities|FlowControl|Delay 4.0)
  (Game|OpenLevel(byName) "GameOver"))

(event EventEyeDamaged
  ;[1 1 1] ダメージ状態の処理（BP側）
  (bind _asbp_vrsmart_phone (Utilities|Casting|CastToBP_VRSmartPhone (Variables|Default|Getvr_Phone)))
  (Default|EyeDamaged _asbp_vrsmart_phone))

(event Input|ActionEvents|InputActionCameraCollisionGenerate
  (params (Key :type Key%20Structure :default "None"))
  ;[1 1 1] カメラの撮影対象判定処理
)

(event Input|ActionEvents|InputActionResetHeight
  (params (Key :type Key%20Structure :default "None"))
  (bind _deviceposition (Class|HeadMountedDisplayFunctionLibrary|GetOrientationandPosition))
  (bind _playerheight (Variables|Default|GetPlayerHeight))
  (bind _returnvalue (- _playerheight (.z _deviceposition)))
  ;[1 1 1] VRモードの時、プレイヤー立っているの高さを設定
  (:Pressed
    (if (Variables|Default|Getvr_isVRmode)
      (Variables|Default|Setm_VRPlayersHeight (.z _deviceposition))
      (Variables|Default|SetVR_Players_Height _returnvalue)
      (Transformation|SetRelativeLocation (Variables|Default|Getm_pCameraBase) (Math|Vector|MakeVector 0.0 0.0 _returnvalue) false false))))

(event Input|ActionEvents|InputActionPlayerSquat
  (params (Key :type Key%20Structure :default "None"))
  ;[1 1 1] PCモード　しゃがむの処理
  (:Pressed
    (if (not (Class|HeadMountedDisplayFunctionLibrary|IsHeadMountedDisplayEnabled))
      (if (Variables|Default|Getcan_player_move_control_)
        (if (not (Variables|Default|GetisCrouching_PC))
          (if (Variables|Default|GetbIsCrouched)
            (Variables|/Script/Engine.SpringArmComponent|SetbEnableCameraLag (Variables|Default|Getm_pSpringArm) true)
            (Character|UnCrouch)
            (Utilities|FlowControl|Delay 0.05)
            (if (not (Variables|Default|GetbIsCrouched))
              (Variables|Default|SetisCrouching_PC true)
              (Variables|Default|Setm_isStanding true)
              (Variables|Default|Setm_isCrouch_PC false)
              (Utilities|SetPlayerCameraHeight (Variables|Default|GetPlayerHeight)
                (:execOut
                  (Audio|PlaySound2D "/Game/SE/Stand.Stand" 1.0 1.0 0.0 0 0)
                  (Utilities|FlowControl|Delay (Variables|Default|GetCrouchCoolTime_PC))
                  (Variables|/Script/Engine.SpringArmComponent|SetbEnableCameraLag (Variables|Default|Getm_pSpringArm) false)
                  (Variables|Default|SetisCrouching_PC false))))
            (else
              (Variables|/Script/Engine.SpringArmComponent|SetbEnableCameraLag (Variables|Default|Getm_pSpringArm) true)
              (Character|Crouch)
              (Variables|Default|SetisCrouching_PC true)
              (Variables|/Script/Engine.SpringArmComponent|SetbEnableCameraLag (Variables|Default|Getm_pSpringArm) true)
              (Variables|Default|Setm_isStanding false)
              (Variables|Default|Setm_isCrouch_PC true)
              (Utilities|SetPlayerCameraHeight (/ (Variables|Default|GetPlayerHeight) (Variables|Default|GetNumToDevideWhenChrouch))
                (:execOut
                  (Audio|PlaySound2D "/Game/SE/Squat.Squat" 1.0 1.0 0.0 0 0)
                  (Utilities|FlowControl|Delay (Variables|Default|GetCrouchCoolTime_PC))
                  (Variables|/Script/Engine.SpringArmComponent|SetbEnableCameraLag (Variables|Default|Getm_pSpringArm) false)
                  (Variables|Default|SetisCrouching_PC false))))))))))

(event Input|ActionEvents|InputActionResetVR
  (params (Key :type Key%20Structure :default "None"))
  (:Pressed
    (Class|HeadMountedDisplayFunctionLibrary|ResetOrientationandPosition 0.0 "OrientationAndPosition")))

(event Input|ActionEvents|InputActionVRCameraTurnRight
  (params (Key :type Key%20Structure :default "None"))
  ;[1 1 1] VR Turn Camera By Button
  (:Pressed
    (Transformation|AddLocalRotation (Variables|Default|Getm_pCameraBase) "0,45.000000, 0" false false)))

(event Input|ActionEvents|InputActionVRCameraTurnLeft
  (params (Key :type Key%20Structure :default "None"))
  ;[1 1 1] VR Turn Camera By Button
  (:Pressed
    (Transformation|AddRelativeRotation (Variables|Default|Getm_pCameraBase) "0,-45.000000, 0" false false)))

(event Input|ActionEvents|InputActionSpeedUp
  (params (Key :type Key%20Structure :default "None"))
  (:Pressed
    (if (< (+ (Variables|Default|Getplayer_run_speed_) 1e+02) 2.5e+03)
      (bind _output_get (Variables|Default|Setplayer_run_speed_ (+ (Variables|Default|Getplayer_run_speed_) 1e+02)))
      (Variables|Default|Setplayer_walk_speed_ (/ _output_get 2.0)))))

(event Input|ActionEvents|InputActionSpeedDown
  (params (Key :type Key%20Structure :default "None"))
  (:Pressed
    (if (> (- (Variables|Default|Getplayer_run_speed_) 1e+02) 701.0)
      (bind _output_get (Variables|Default|Setplayer_run_speed_ (- (Variables|Default|Getplayer_run_speed_) 1e+02)))
      (Variables|Default|Setplayer_walk_speed_ (/ _output_get 2.0)))))

(event Input|KeyboardEvents|M
  (params (Key :type Key%20Structure :default "None"))
  ;[1 1 1] VR Turn Camera By Button
)

(event Input|KeyboardEvents|N
  (params (Key :type Key%20Structure :default "None"))
  ;[1 1 1] VR Turn Camera By Button
)

(fn ConstructionScript)

(fn CheckNottheTargettoBlackOut
  (params (InputClass :type Actor%20Class%20Reference))
  (return (Math|Boolean|ORBoolean (Utilities|ClassIsChildOf InputClass 0) (Utilities|ClassIsChildOf InputClass "/Game/Blueprints/BP_AutomaticDoorLever.BP_AutomaticDoorLever_C") (Utilities|ClassIsChildOf InputClass "/Game/Blueprints/BP_CardKey.BP_CardKey_C"))))

(fn CheckCameratoPlayerDistance
  (params (MaxDistance :type Float%20%28single-precision%29))
  (bind _m_pcamera (Variables|Default|Getm_pCamera))
  (bind _capsulecomponent (Variables|Default|GetCapsuleComponent))
  (bind _returnvalue (Transformation|GetWorldLocation _m_pcamera))
  (bind _returnvalue_2 (Transformation|GetWorldLocation _capsulecomponent))
  (return (> (.OutLength (Class|KismetMathLibrary|ToDirectionandLength2D (- (Math|Vector2D|MakeVector2D (.x _returnvalue) (.y _returnvalue)) (Math|Vector2D|MakeVector2D (.x _returnvalue_2) (.y _returnvalue_2))))) MaxDistance)))