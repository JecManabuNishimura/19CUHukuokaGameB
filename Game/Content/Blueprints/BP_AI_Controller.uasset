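; AI controller for BP_AI_Enemy that starts its behavior tree and supplies waypoint patrol movement.
; On BeginPlay it copies the pawn's patrol points, writes its wait duration to the BB_Enemy blackboard and runs BT_Enemy; boss tree nodes are unconnected.
; GoToPatrol, not called here, moves to the current point, advances cyclically and re-arms by timer on success.
; GetPatrolLocation returns the cached previous location when any coordinate is zero.
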(event Custom|GoToPatrol
  (AI|AIMoveTo (Pawn|GetControlledPawn) (CallFunction|GetPatrolLocation) 0 5.0 false
    (:OnSuccess
      (CallFunction|PopPatrolLocation)
      (Utilities|Time|SetTimerbyFunctionName 0 "GoToPatrol" 0.1))))

(event EventBeginPlay
  (bind _asbp_ai_enemy (Utilities|Casting|CastToBP_AI_Enemy (Pawn|GetControlledPawn)))
  (Variables|Default|SetAI_PatrolPoints (Variables|/Game/Blueprints/BP_AI_Enemy.BP_AI_Enemy_C|GetPatrolPoints _asbp_ai_enemy))
  (Class|AIController|UseBlackboard "/Game/BT/BB_Enemy.BB_Enemy")
  (AI|Components|Blackboard|SetValueasFloat (AI|GetBlackboard 0) (Utilities|Name|MakeLiteralName "PatrolWaitDuration") (Variables|/Game/Blueprints/BP_AI_Enemy.BP_AI_Enemy_C|GetPatrolWaitDuration _asbp_ai_enemy))
  (AI|RunBehaviorTree "/Game/BT/BT_Enemy.BT_Enemy"))

(event EventTick
  (params (DeltaSeconds :type Float%20%28single-precision%29)))

(fn ConstructionScript)

(fn PopPatrolLocation
  (Variables|Default|SetPatrolPoint (Math|Integer|%(Integer) (+ (Variables|Default|GetPatrolPoint) 1) (Utilities|Array|Length (Variables|Default|GetAI_PatrolPoints)))))

(fn GetPatrolLocation
  (bind _ai_patrolpoints (Variables|Default|GetAI_PatrolPoints))
  (bind _patrolpoint (Variables|Default|GetPatrolPoint))
  (bind _output (Utilities|Array|Get(acopy) _ai_patrolpoints _patrolpoint))
  (bind _returnvalue (Transformation|GetActorLocation _output))
  (if (Utilities|IsValid _output)
    (if (Math|Boolean|ORBoolean (== (.x _returnvalue) 0.0) (== (.y _returnvalue) 0.0) (== (.z _returnvalue) 0.0))
      (return (Variables|Default|GetprebLocation))
      (else
        (Variables|Default|SetprebLocation (Math|Vector|MakeVector (.x _returnvalue) (.y _returnvalue) (.z _returnvalue)))
        (return (Math|Vector|MakeVector (.x _returnvalue) (.y _returnvalue) (.z _returnvalue)))))))