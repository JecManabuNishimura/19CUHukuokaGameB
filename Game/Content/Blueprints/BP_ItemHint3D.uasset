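; BP_ItemHint3D is a floating 3D hint widget actor for VR items, shown only when the player is near.
; Each Tick measures distance to the player's MPCamera, toggles widget visibility and smoothly turns the actor toward the camera.
; Inside a closer threshold the widget eases up to a working height, and sinks back outside it.
; Initial functions let callers set that height, the widget scale and the threshold.
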(event EventBeginPlay
  (bind _asbp_player_character (Utilities|Casting|CastToBP_PlayerCharacter (Game|GetPlayerCharacter 0)))
  (Variables|Default|SetPlayer1 _asbp_player_character)
  (CallFunction|CheckPlayerRef)
  (bind _asvr_item_hint (Utilities|Casting|CastToVR_ItemHint (UserInterface|GetUserWidgetObject (Variables|Default|GetVR_ItemCommandWidget))))
  (Variables|Default|SetVR_ItemHintWidget _asvr_item_hint)
  (Transformation|SetActorRotation (Utilities|GetRotationfromActortoCamera))
  (Rendering|SetVisibility (Variables|Default|GetVR_ItemCommandWidget) false false))

(event Collision|EventActorBeginOverlap
  (params (OtherActor :type Actor%20Object%20Reference)))

(event EventTick
  (params (DeltaSeconds :type Float%20%28single-precision%29))
  (Utilities|GetDistancetoPlayer
    (:Out
      (if (< (Variables|Default|GetCurrentDistance) (Variables|Default|GetVisableDistance))
        (Rendering|SetVisibility (Variables|Default|GetVR_ItemCommandWidget) true false)
        (Transformation|SetActorRotation (Math|Interpolation|RInterpTo (Transformation|GetActorRotation) (Utilities|GetRotationfromActortoCamera) DeltaSeconds 3e+01))
        (if (< (Variables|Default|GetCurrentDistance) (Variables|Default|GetbetweenToPlayersDistance))
          (if (< (.z (Variables|/Script/Engine.SceneComponent|GetRelativeLocation (Variables|Default|GetVR_ItemCommandWidget))) (Variables|Default|GetWorkingHeight))
            (Transformation|SetRelativeLocation (Variables|Default|GetVR_ItemCommandWidget) (Math|Interpolation|VInterpTo (Variables|/Script/Engine.SceneComponent|GetRelativeLocation (Variables|Default|GetVR_ItemCommandWidget)) (Math|Vector|MakeVector 0.0 0.0 (Variables|Default|GetWorkingHeight)) DeltaSeconds 3.0) false false))
          (elif (> (.z (Variables|/Script/Engine.SceneComponent|GetRelativeLocation (Variables|Default|GetVR_ItemCommandWidget))) 1.0)
            (Transformation|SetRelativeLocation (Variables|Default|GetVR_ItemCommandWidget) (Math|Interpolation|VInterpTo (Variables|/Script/Engine.SceneComponent|GetRelativeLocation (Variables|Default|GetVR_ItemCommandWidget)) "0, 0, 0" DeltaSeconds 3.0) false false)))
        (else
          (Rendering|SetVisibility (Variables|Default|GetVR_ItemCommandWidget) false false))))))

(fn ConstructionScript)

(fn CheckPlayerRef
  (bind _returnvalue (Game|GetPlayerCharacter 0))
  (if (Utilities|IsValid (Variables|Default|GetPlayer1))
    (return)
    (elif (Utilities|IsValid _returnvalue)
      (bind _asbp_player_character (Utilities|Casting|CastToBP_PlayerCharacter _returnvalue)
        (:then
          (Variables|Default|SetPlayer1 _asbp_player_character)
          (if (Utilities|IsValid (Variables|Default|GetPlayer1))
            (return)
            (else
              (Development|PrintString "Failed To Acess  BP_PlayerCharacter" true true "(R=1.000000,G=0.000000,B=0.109215,A=1.000000)" 5.0))))
        (:CastFailed
          (Development|PrintString "Cast Failed of BP_PlayerCharacter" true true "(R=1.000000,G=0.000000,B=0.109215,A=1.000000)" 5.0)))
      (else
        (Development|PrintString "Can't Get Player in VRSmartPhone" true true "(R=1.000000,G=0.000000,B=0.109215,A=1.000000)" 5.0)))))

(fn InitialHeight
  (params (Height :type Float%20%28single-precision%29))
  (Variables|Default|SetWorkingHeight Height))

(fn InitialScale
  (params (Scale :type Float%20%28single-precision%29))
  (Transformation|SetWorldScale3D (Variables|Default|GetVR_ItemCommandWidget) (Math|Vector|MakeVector Scale Scale Scale)))

(fn InitialDistance
  (params (Distance :type Float%20%28single-precision%29))
  (Variables|Default|SetbetweenToPlayersDistance Distance))