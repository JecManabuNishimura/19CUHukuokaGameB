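; Stationary fluorescent light actor that powers up on BeginPlay, then flickers with sound.
; An intro timeline drives a rect light and the emissive power of one dynamic material shared by two meshes.
; When it finishes, FlashingType picks a blink pattern, whose timeline starts at a random offset, updates both outputs and fires sounds at the actor.
; A third, silent blink pattern exists but is never triggered.
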(event EventBeginPlay
  (|SetDMI)
  (bind _新規track_0 (Timeline|タイムライン_1 Play)
    (:Update
      (Variables|Default|Setintensity _新規track_0)
      (Rendering|Material|SetScalarParameterValue (Variables|Default|GetDynamic%20Material) "MI_FLightPower" (Variables|Default|Getintensity) :!class /Script/Engine.MaterialInstanceDynamic)
      (Rendering|Components|Light|SetIntensity (Variables|Default|GetRectLight) (Variables|Default|Getintensity)))
    (:Finished
      (switch int (Variables|Default|GetFlashing_Type)
        (:Default
          (|Blinking0 :!label _label
            (:Update
              _)))
        (:0
          (goto _label))
        (:1
          (|Blinking1
            (:Update
              _))))
      (Rendering|Material|SetScalarParameterValue (Variables|Default|GetDynamic%20Material) "MI_FLightPower" (Variables|Default|Getintensity) :!class /Script/Engine.MaterialInstanceDynamic)
      (Rendering|Components|Light|SetIntensity (Variables|Default|GetRectLight) (* (Variables|Default|Getintensity) 1.25)))))

(event EventTick
  (params (DeltaSeconds :type Float%20%28single-precision%29)))

(fn ConstructionScript)