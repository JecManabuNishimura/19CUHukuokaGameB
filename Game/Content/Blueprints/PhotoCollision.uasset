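; Short-lived photo-shot collision actor that detects photographed targets and advances photo missions.
; A mesh overlap with a PhotoTargetActor-tagged BP_AI_Enemy triggers a camera-oriented box trace on the TakePhotoCollision profile.
; Any trace hit lets an enemy with a mission number update BP_PlayerCharacter's mission and be marked complete, then the actor self-destructs.
; Tick drives a delayed failure message and destruction while nothing is hit.
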(event OnComponentBeginOverlap(StaticMesh)
  (params (OverlappedComponent :type Primitive%20Component%20Object%20Reference) (OtherActor :type Actor%20Object%20Reference) (OtherComp :type Primitive%20Component%20Object%20Reference) (OtherBodyIndex :type Integer) (bFromSweep :type Boolean) (SweepResult :type Hit%20Result%20Structure%20%28by%20ref%29))
  (bind _returnvalue (Game|GetPlayerCameraManager 0))
  (bind _returnvalue_2 (Transformation|GetActorLocation))
  (bind _returnvalue_3 (Transformation|GetActorForwardVector _returnvalue))
  (if (not (Variables|Default|GetisHit))
    (if (Actor|ActorHasTag OtherActor "PhotoTargetActor")
      (Variables|Default|SetisHit true)
      (if (== (Utilities|GetClass OtherActor) "/Game/Blueprints/BP_AI_Enemy.BP_AI_Enemy_C")
        (bind _asbp_ai_enemy (Utilities|Casting|CastToBP_AI_Enemy OtherActor))
        (if (Variables|/Game/Blueprints/BP_AI_Enemy.BP_AI_Enemy_C|GetisMissionComplete _asbp_ai_enemy)
          (Variables|Default|SetisHit false)
          (else
            (Development|PrintString "23333333333333333333")
            (bind (_outhit _returnvalue_4) (Class|KismetSystemLibrary|BoxTraceSinglebyProfile (+ _returnvalue_2 (* _returnvalue_3 2e+02)) (+ _returnvalue_2 (* _returnvalue_3 (Variables|Default|GetCameraDistanceRangeMAX))) "50.000000,80.000000,100.000000" (Camera|GetCameraRotation _returnvalue) "TakePhotoCollision" false (Utilities|Array|MakeArray (Game|Player|GetPlayerPawn 0)) "None" true "(R=1.000000,G=0.000000,B=0.000000,A=1.000000)" "(R=0.000000,G=1.000000,B=0.000000,A=1.000000)" 1.0))
            (if _returnvalue_4
              (Development|PrintString (Utilities|GetDisplayName (.HitActor (Collision|BreakHitResult _outhit))) true true "(R=1.000000,G=0.781673,B=0.000000,A=1.000000)" 5.0)
              (if (> (Variables|/Game/Blueprints/BP_AI_Enemy.BP_AI_Enemy_C|Getitems_Mission_Num _asbp_ai_enemy) 0)
                (bind _asbp_player_character (Utilities|Casting|CastToBP_PlayerCharacter (Game|Player|GetPlayerPawn 0)))
                (bind __hasupdated (Class|PlayerCharacter|UpdatetheMission _asbp_player_character 2 (Variables|/Game/Blueprints/BP_AI_Enemy.BP_AI_Enemy_C|Getitems_Mission_Num _asbp_ai_enemy)))
                (if __hasupdated
                  (Variables|/Game/Blueprints/BP_AI_Enemy.BP_AI_Enemy_C|SetisMissionComplete _asbp_ai_enemy true)))
              (Utilities|FlowControl|Delay 1.0)
              (Actor|DestroyActor)
              (else
                (Variables|Default|SetisHit false)))))))))

(event EventBeginPlay)

(event Collision|EventActorBeginOverlap
  (params (OtherActor :type Actor%20Object%20Reference)))

(event EventTick
  (params (DeltaSeconds :type Float%20%28single-precision%29))
  (if (not (Variables|Default|GetisHit))
    (Utilities|FlowControl|Delay 1.0)
    (Development|PrintString "Shooting failure..." true false "(R=0.000000,G=1.000000,B=0.000000,A=1.000000)")
    (Actor|DestroyActor)))

(fn ConstructionScript)