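; Tutorial level game mode that scripts the opening and ending of the tutorial.
; BeginPlay moves the player to a placed start-position actor, locks input, polls until BP_VRSmartPhone exists, then hides it and shows the dialogue widget.
; DialogueEnd plays timed footstep and door sounds, sets CanLightOn, reveals the phone and restores input.
; FloorCollapse hides the phone, disables input and loads the Master level after a delay.
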(event Custom|FloorCollapse
  (Rendering|SetActorHiddenInGame (Variables|Default|GetSmartphone) true)
  (Input|DisableInput (Game|GetPlayerCharacter 0) (Game|GetPlayerController 0))
  (Utilities|FlowControl|Delay 4.0)
  (Game|OpenLevel(byName) "Master"))

(event Custom|DialogueEnd
  (|MakeFootStepAuto)
  (Audio|PlaySound2D "/Game/SE/Door_Open_1.Door_Open_1" 1.0 1.0 0.0 0 0)
  (Utilities|FlowControl|Delay 1.5)
  (|MakeFootStepAuto_2)
  (Audio|PlaySound2D "/Game/SE/Door_Close_1.Door_Close_1" 1.0 1.0 0.0 0 0)
  (Utilities|FlowControl|Delay 1.0)
  (Variables|Default|SetcanLightOn true)
  (Utilities|FlowControl|Delay 2.0)
  (Rendering|SetActorHiddenInGame (Variables|Default|GetSmartphone) false)
  (Utilities|FlowControl|Delay 1.0)
  (Input|EnableInput (Game|GetPlayerCharacter 0) (Game|GetPlayerController 0)))

(event EventBeginPlay
  (bind _returnvalue (Game|GetPlayerCharacter 0))
  ;[1 1 1] プレイヤーの初期位置設定(PlayerInitialPosActorの座標、回転情報をPlayerCharacterに渡す)
  (bind _returnvalue_2 (Actor|GetActorOfClass "/Game/Blueprints/PlayerInitialPosActor.PlayerInitialPosActor_C"))
  (Utilities|IsValid _returnvalue_2
    (:Is%20Valid
      (Utilities|IsValid _returnvalue
        (:Is%20Valid
          (Transformation|SetActorTransform _returnvalue (Math|Transform|MakeTransform (.location (Transformation|GetActorTransform _returnvalue_2)) (.rotation (Transformation|GetActorTransform _returnvalue_2)) "1,1,1"))
          (Actor|DestroyActor _returnvalue_2)
          (Variables|Default|SetcanLightOn false)
          (Input|DisableInput (Game|GetPlayerCharacter 0) (Game|GetPlayerController 0))
          (Utilities|FlowControl|Delay 0.01 :!label _label)
          (bind _outactors (Actor|GetAllActorsOfClass "/Game/Blueprints/BP_VRSmartPhone.BP_VRSmartPhone_C"))
          (if (!= (Utilities|Array|Length _outactors) 0)
            (bind _array_element (Utilities|Array|ForEachLoopwithBreak _outactors)
              (:LoopBody
                (bind _output_get (Variables|Default|SetSmartphone _array_element))
                (Rendering|SetActorHiddenInGame _output_get true))
              (:Completed
                (bind _returnvalue_3 (UserInterface|CreateWidget "/Game/UI/TutorialDialogue.TutorialDialogue_C"))
                (bind _output_get_2 (Variables|Default|SetDialogueWidget _returnvalue_3))
                (UserInterface|Viewport|AddtoViewport _output_get_2 0)))
            (else
              (goto _label))))))))

(event EventTick
  (params (DeltaSeconds :type Float%20%28single-precision%29)))

(fn ConstructionScript)