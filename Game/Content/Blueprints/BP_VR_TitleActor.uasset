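; BP_VR_TitleActor is a VR title label actor whose widget background is resized to fit a text string.
; CalAndGiveSizeOfBackground gets the string's byte length from the player, divides it by three, and scales it by a per-word width plus padding at fixed height.
; CheckPlayerRef caches the BP_PlayerCharacter reference, printing errors on failure.
; The event graph is empty, and a look-at-camera rotation calculation is left unused.
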(event Collision|EventActorBeginOverlap
  (params (OtherActor :type Actor%20Object%20Reference)))

(fn ConstructionScript)

(fn CheckPlayerRef
  (bind _returnvalue (Game|GetPlayerCharacter 0))
  (if (Utilities|IsValid (Variables|Default|GetPlayer1))
    (return)
    (elif (Utilities|IsValid _returnvalue)
      (bind _asbp_player_character (Utilities|Casting|CastToBP_PlayerCharacter _returnvalue)
        (:then
          (Variables|Default|SetPlayer1 _asbp_player_character)
          (if (Utilities|IsValid (Variables|Default|GetPlayer1))
            (return)
            (else
              (Development|PrintString "Failed To Acess  BP_PlayerCharacter" true true "(R=1.000000,G=0.000000,B=0.109215,A=1.000000)" 5.0))))
        (:CastFailed
          (Development|PrintString "Cast Failed of BP_PlayerCharacter" true true "(R=1.000000,G=0.000000,B=0.109215,A=1.000000)" 5.0)))
      (else
        (Development|PrintString "Can't Get Player in VRSmartPhone" true true "(R=1.000000,G=0.000000,B=0.109215,A=1.000000)" 5.0)))))