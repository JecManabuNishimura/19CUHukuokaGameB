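; Enemy AI character that senses the player by sight and sound and holds the resulting state behind getter and setter functions.
; PawnSensing sets a seen flag or records the player on any heard noise, while the AttackRange sensor flags the player as found.
; CreateRay line-traces from above the enemy to the player for obstructions.
; Helpers set walk speed and switch mutually exclusive idle, walk, run and attack animation booleans.
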(event OnHearNoise(PawnSensing)
  (params (Instigator :type Pawn%20Object%20Reference) (Location :type Vector%20%28by%20ref%29 :default "0, 0, 0") (Volume :type Float%20%28single-precision%29))
  ;[1 1 1] ノイズが入った際の処理
  (Development|PrintString (Utilities|String|Append "音の出した対象と位置と音量：" (Utilities|GetObjectName Instigator) "&" (Utilities|String|ToString(Vector) Location) "&" (Utilities|String|ToString(Float) Volume)) true true "(R=0.000000,G=0.660000,B=1.000000,A=1.000000)" (stale EventTick DeltaSeconds))
  (Variables|Default|SetisHearNoisePawn (Variables|Default|Getplayer)))

(event OnSeePawn(PawnSensing)
  (params (Pawn :type Pawn%20Object%20Reference))
  ;[1 1 1] Playerを発見した時に処理
  (Variables|Default|Setseeflag true)
  (CallFunction|IsSeePlayerActor Pawn)
  (Development|PrintString "SeePlayer" true true "(R=0.000000,G=0.660000,B=1.000000,A=1.000000)" (stale EventTick DeltaSeconds)))

(event OnComponentHit(CapsuleComponent)
  (params (HitComponent :type Primitive%20Component%20Object%20Reference) (OtherActor :type Actor%20Object%20Reference) (OtherComp :type Primitive%20Component%20Object%20Reference) (NormalImpulse :type Vector :default "0, 0, 0") (Hit :type Hit%20Result%20Structure%20%28by%20ref%29))
  ;[1 1 1] Playerがぶつかった時の処理
)

(event OnSeePawn(AttackRange)
  (params (Pawn :type Pawn%20Object%20Reference))
  ;[1 1 1] 攻撃範囲内に入った時の処理
  (CallFunction|IsSeePlayerActor Pawn)
  (Development|PrintString "isAttack = true" true true "(R=0.000000,G=0.660000,B=1.000000,A=1.000000)" (stale EventTick DeltaSeconds))
  (bind _asplayer_character (Utilities|Casting|CastToPlayerCharacter Pawn))
  (Class|PlayerCharacter|SetIsFound _asplayer_character true))

(event EventTick
  (params (DeltaSeconds :type Float%20%28single-precision%29)))

(event EventBeginPlay
  ;[1 1 1] 歩く速度の初期化
  (CallFunction|SetWalkSpeed (Variables|Default|GetenemyWalkSpeed))
  (Variables|Default|Setplayer (Game|GetPlayerCharacter 0)))

(fn ConstructionScript)

(fn CanSeePlayerPawn
  (bind _returnvalue (Transformation|GetActorLocation))
  (bind _outhit (Collision|LineTraceByChannel _returnvalue (+ _returnvalue (* (Transformation|GetActorForwardVector) (Variables|Default|GetSightLength))) "TraceTypeQuery3" false 0 "ForOneFrame"))
  (Utilities|IsValid (.HitActor (Collision|BreakHitResult _outhit))
    (:Is%20Valid
      (return (Actor|ActorHasTag (.HitActor (Collision|BreakHitResult _outhit)) "Player") (.HitActor (Collision|BreakHitResult _outhit))))))

(fn IsSeePlayerActor
  (params (SeePlayer :type Actor%20Object%20Reference))
  (bind _output_get (Variables|Default|SetIsSeePlayer false))
  (Variables|Default|SetSeePlayer SeePlayer)
  (if _output_get
    _))

(fn CanSeePlayer
  (return (Variables|Default|Getseeflag)))

(fn SetCanSeeFlag
  (params (flag :type Boolean))
  (Variables|Default|Setseeflag flag))

(fn CreateRay
  (bind _returnvalue (Transformation|GetActorLocation))
  (bind _returnvalue_2 (Collision|LineTraceByChannel (Math|Vector|MakeVector (.x _returnvalue) (.y _returnvalue) (+ (.z _returnvalue) 2e+02)) (Transformation|GetActorLocation (Variables|Default|Getplayer)) "TraceTypeQuery1" false 0 "ForDuration")) ; 壁を挟んでいたら(間に物があったら)true
  (return (not _returnvalue_2)))

(fn SetWalkSpeed
  (params (NewParam :type Float%20%28single-precision%29))
  (bind _output_get (Variables|/Script/Engine.CharacterMovementComponent|SetMaxWalkSpeed (Variables|Character|GetCharacterMovement) NewParam))
  (Development|PrintString (Utilities|String|Append "EnemySpeed is" (Utilities|String|ToString(Float) _output_get))))

(fn MakedNoisePawn
  (params (NewParam :type Actor%20Object%20Reference))
  (Variables|Default|SetisHearNoisePawn NewParam))

(fn SetAnimationAttack
  (Variables|Default|SetAnimation_Attack true)
  (Variables|Default|SetAnimation_Idle false)
  (Variables|Default|SetAnimation_Run false)
  (Variables|Default|SetAnimation_Walk false))

(fn SetAnimationIdle
  (Variables|Default|SetAnimation_Attack false)
  (Variables|Default|SetAnimation_Idle true)
  (Variables|Default|SetAnimation_Run false)
  (Variables|Default|SetAnimation_Walk false))

(fn SetAnimationRun
  (Variables|Default|SetAnimation_Attack false)
  (Variables|Default|SetAnimation_Idle false)
  (Variables|Default|SetAnimation_Run true)
  (Variables|Default|SetAnimation_Walk false))

(fn SetAnimationWalk
  (Variables|Default|SetAnimation_Attack false)
  (Variables|Default|SetAnimation_Idle false)
  (Variables|Default|SetAnimation_Run false)
  (Variables|Default|SetAnimation_Walk true))

(fn GetAnimationIdle
  (return (Variables|Default|GetAnimation_Idle)))

(fn GetAnimationRun
  (return (Variables|Default|GetAnimation_Run)))

(fn GetAnimationWalk
  (return (Variables|Default|GetAnimation_Walk)))

(fn GetAnimationAttack
  (return (Variables|Default|GetAnimation_Attack)))