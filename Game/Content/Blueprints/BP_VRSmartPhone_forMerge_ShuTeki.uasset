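; VR smartphone actor that cycles camera, flashlight, mission and heartbeat apps on a widget switcher via key, gamepad and VR inputs.
; Camera mode zooms by FOV and briefly shows snapshots drawn to a render target.
; Mission text comes from a DataTable by the player's mission number, with screen layout chosen by HMD state.
; Tick animates the heartbeat, changing pulse rate and size when the enemy is within alarm distance.
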(event EventBeginPlay
  (Input|EnableInput (Game|GetPlayerController 0))
  (bind _outactors (Actor|GetAllActorsOfClass "/Script/hukuokaGame.PlayerCharacter"))
  (for (_array_element _array_index) _outactors
    (if (not (Math|Conversions|ToBoolean(Integer) _array_index))
      (Variables|Default|Setplayer1 _array_element)
      ;[1 1 1] Get the VR_SmartPhoneUI object
      (bind _asvrsmart_phone_widget (Utilities|Casting|CastToVRsmartPhoneWidget (UserInterface|GetUserWidgetObject (Variables|Default|GetSmartPhoneUIWidget))))
      (Variables|Default|SetVRSmartPhoneUI _asvrsmart_phone_widget)
      (bind _returnvalue (Actor|GetActorOfClass "/Game/Blueprints/BP_PlayerCharacter.BP_PlayerCharacter_C"))
      (Variables|Default|SetPlayerCharaterRef _returnvalue))))

(event Collision|EventActorBeginOverlap
  (params (OtherActor :type Actor%20Object%20Reference)))

(event EventTick
  (params (DeltaSeconds :type Float%20%28single-precision%29))
  (bind _heartbeat_isappon (Variables|Default|GetHeartBeat_isAppOn))
  (bind _vrsmartphoneui (Variables|Default|GetVRSmartPhoneUI))
  ;[1 1 1] for Changing App's time counting
  (if (Variables|Default|GetisLoadingAPP)
    (bind _returnvalue (Rendering|Material|GetScalarParameterValue 0 "None" :!class /Script/Engine.KismetMaterialLibrary))
    (Rendering|Material|SetScalarParameterValue 0 "NowTime" (+ _returnvalue DeltaSeconds) :!class /Script/Engine.KismetMaterialLibrary)
    (elif (Variables|Default|GetLighyUI_isShowing)
      (CallFunction|UIDisappearingFunc DeltaSeconds (Variables|Default|GetdisAppearingImage))
      (else
        (if (< (Transformation|GetDistanceTo (Utilities|ResolveSoftReference (Variables|Default|GetenemyRef))) (Variables|Default|GetalarmDistance))
          ;[1 1 1] 心拍数のパラメータの変更
          (Variables|Default|SetHeartBeat_beatDelay 1.0)
          (Variables|Default|SetHeartBeat_scaleSize 1.4)
          (else
            (Variables|Default|SetHeartBeat_beatDelay 2.0)
            (Variables|Default|SetHeartBeat_scaleSize 1.2)))
        ;[1 1 1] 心拍アニメーション by_朱
        (if (and (Variables|Default|GetHearBeat_isNotDamaged) _heartbeat_isappon)
          (Utilities|FlowControl|Delay (Variables|Default|GetHeartBeat_beatDelay))
          (if _heartbeat_isappon
            (if (Variables|Default|GetHeartBeat_isScaling)
              (Default|HeartBeatAnimate _vrsmartphoneui 1.0)
              (Variables|Default|SetHeartBeat_isScaling false)
              (else
                (Default|HeartBeatAnimate _vrsmartphoneui (Variables|Default|GetHeartBeat_scaleSize))
                (Variables|Default|SetHeartBeat_isScaling true)))))))))

(event Input|ActionEvents|InputActionGrabRight
  (params (Key :type Key%20Structure :default "None"))
  ;[1 1 1] VRのスマホライトOn/Off  / Change VR Smart Phone Camera Light on/off
  (:Pressed
    (if (== (Variables|Default|GetSmartPhoneMode) 1)
      (if (Variables|Default|GetCameraLightOn)
        (Rendering|SetVisibility (Variables|Default|GetCameraLight) false false)
        (Rendering|SetVisibility (Variables|Default|GetCameraLight2) false false)
        (Variables|Default|SetCameraLightOn false)
        (CallFunction|SetLightUIONOFF false)
        (else
          (Rendering|SetVisibility (Variables|Default|GetCameraLight) true false)
          (Rendering|SetVisibility (Variables|Default|GetCameraLight2) true false)
          (Variables|Default|SetCameraLightOn true)
          (CallFunction|SetLightUIONOFF true))))))

(event Input|ActionEvents|InputActionHeartBeatStatusSwitch
  (params (Key :type Key%20Structure :default "None"))
  ;[1 1 1] HeartBeatアプリのOn/Off　 by_朱
  (:Pressed
    (if (Variables|Default|GetHearBeat_isNotDamaged)
      (CallFunction|HeartBeatStatusSwitch))))

(event Input|ActionEvents|InputActionGrabRight
  (params (Key :type Key%20Structure :default "None"))
  ;[1 1 1] Change VR Smart Phone's display's material  when  took a photo.  It will display [Photo_ShowOutTime] seconds and change back to live mode.
  (:Pressed
    (if (== (Variables|Default|GetSmartPhoneMode) 0)
      (if (Variables|/Script/hukuokaGame.PlayerCharacter|Getvr_InCameraMode (Variables|Default|Getplayer1))
        _
        (else
          _))
      (Rendering|ClearRenderTarget2D "/Game/Materials/photoTarget.photoTarget" "(R=0.000000,G=0.000000,B=0.000000,A=255.000000)")
      (Rendering|DrawMaterialtoRenderTarget "/Game/Materials/photoTarget.photoTarget" "/Game/Materials/smartPhoneDisplay.SmartPhoneDisplay")
      (Variables|Default|SetisShowingPhoto true)
      (CallFunction|SetCameraUIONOFF (Variables|Default|GetVRSmartPhoneUI) false)
      (Rendering|Material|SetMaterial (Variables|Default|GetVRSmartPhoneDisplay) 0 "/Game/Materials/PhotoDisplay.PhotoDisplay")
      (Utilities|FlowControl|Delay (Variables|Default|GetPhoto_ShowOutTime))
      (Rendering|Material|SetMaterial (Variables|Default|GetVRSmartPhoneDisplay) 0 "/Game/Materials/smartPhoneDisplay.SmartPhoneDisplay")
      (Variables|Default|SetisShowingPhoto false)
      (CallFunction|SetCameraUIONOFF (Variables|Default|GetVRSmartPhoneUI) true))))

(event Input|ActionEvents|InputActionTriggerLeft
  (params (Key :type Key%20Structure :default "None"))
  (bind _camerafov_default (Variables|Default|GetCameraFOV_default))
  (:Pressed
    (switch int (Variables|Default|GetSmartPhoneMode)
      (:0
        (Variables|Default|SetSmartPhoneMode 1)
        (if (Variables|Default|GetCameraLightOn)
          (CallFunction|SetLightUIONOFF true)
          (else
            (CallFunction|SetLightUIONOFF false)))
        (Class|WidgetSwitcher|SetActiveWidgetIndex (Variables|/Game/UI/VRsmartPhoneWidget.VRsmartPhoneWidget_C|GetDisplaySwitcher (Variables|Default|GetVRSmartPhoneUI)) 1))
      (:1
        (Variables|Default|SetSmartPhoneMode 2)
        (CallFunction|SetMissionContentsSingle)
        (if (Class|HeadMountedDisplayFunctionLibrary|IsHeadMountedDisplayEnabled)
          (Class|WidgetSwitcher|SetActiveWidgetIndex (Variables|/Game/UI/VRsmartPhoneWidget.VRsmartPhoneWidget_C|GetDisplaySwitcher (Variables|Default|GetVRSmartPhoneUI)) 2)
          (else
            (Class|WidgetSwitcher|SetActiveWidgetIndex (Variables|/Game/UI/VRsmartPhoneWidget.VRsmartPhoneWidget_C|GetDisplaySwitcher (Variables|Default|GetVRSmartPhoneUI)) 3))))
      (:2
        (Variables|Default|SetSmartPhoneMode 3)
        (Class|WidgetSwitcher|SetActiveWidgetIndex (Variables|/Game/UI/VRsmartPhoneWidget.VRsmartPhoneWidget_C|GetDisplaySwitcher (Variables|Default|GetVRSmartPhoneUI)) 4)
        (CallFunction|HeartBeatStatusSwitch))
      (:3
        (Variables|Default|SetSmartPhoneMode 0)
        (Class|WidgetSwitcher|SetActiveWidgetIndex (Variables|/Game/UI/VRsmartPhoneWidget.VRsmartPhoneWidget_C|GetDisplaySwitcher (Variables|Default|GetVRSmartPhoneUI)))
        (Variables|/Script/Engine.SceneCaptureComponent2D|SetFOVAngle (Variables|Default|GetVRSmartPhoneCamera) _camerafov_default)
        (Variables|Default|SetCameraFOV_Current _camerafov_default)
        (Variables|Default|SetHeartBeat_isAppOn false)))))

(event Input|KeyboardEvents|X
  (params (Key :type Key%20Structure :default "None"))
  ;[1 1 1] HeartBeatアプリのOn/Off　 by_朱
)

(event Input|KeyboardEvents|C
  (params (Key :type Key%20Structure :default "None"))
  ;[1 1 1] [Not using, for expansion] Save the photo to img_path (need to rotate if want to use)
)

(event Input|GamepadEvents|GamepadLeftTrigger
  (params (Key :type Key%20Structure :default "None"))
  (bind _camerafov_default (Variables|Default|GetCameraFOV_default))
  (:Pressed
    (switch int (Variables|Default|GetSmartPhoneMode)
      (:0
        (Variables|Default|SetSmartPhoneMode 3)
        (Class|WidgetSwitcher|SetActiveWidgetIndex (Variables|/Game/UI/VRsmartPhoneWidget.VRsmartPhoneWidget_C|GetDisplaySwitcher (Variables|Default|GetVRSmartPhoneUI)) 4)
        (CallFunction|HeartBeatStatusSwitch))
      (:1
        (Variables|Default|SetSmartPhoneMode 0)
        (Class|WidgetSwitcher|SetActiveWidgetIndex (Variables|/Game/UI/VRsmartPhoneWidget.VRsmartPhoneWidget_C|GetDisplaySwitcher (Variables|Default|GetVRSmartPhoneUI)))
        (Variables|/Script/Engine.SceneCaptureComponent2D|SetFOVAngle (Variables|Default|GetVRSmartPhoneCamera) _camerafov_default)
        (Variables|Default|SetCameraFOV_Current _camerafov_default)
        (Variables|Default|SetHeartBeat_isAppOn false))
      (:2
        (Variables|Default|SetSmartPhoneMode 1)
        (if (Variables|Default|GetCameraLightOn)
          (CallFunction|SetLightUIONOFF true)
          (else
            (CallFunction|SetLightUIONOFF false)))
        (Class|WidgetSwitcher|SetActiveWidgetIndex (Variables|/Game/UI/VRsmartPhoneWidget.VRsmartPhoneWidget_C|GetDisplaySwitcher (Variables|Default|GetVRSmartPhoneUI)) 1))
      (:3
        (Variables|Default|SetSmartPhoneMode 2)
        (Variables|Default|SetHeartBeat_isAppOn false)
        (CallFunction|SetMissionContentsSingle)
        (if (Class|HeadMountedDisplayFunctionLibrary|IsHeadMountedDisplayEnabled)
          (Class|WidgetSwitcher|SetActiveWidgetIndex (Variables|/Game/UI/VRsmartPhoneWidget.VRsmartPhoneWidget_C|GetDisplaySwitcher (Variables|Default|GetVRSmartPhoneUI)) 2)
          (else
            (Class|WidgetSwitcher|SetActiveWidgetIndex (Variables|/Game/UI/VRsmartPhoneWidget.VRsmartPhoneWidget_C|GetDisplaySwitcher (Variables|Default|GetVRSmartPhoneUI)) 3)))))))

(event Input|GamepadEvents|GamepadFaceButtonBottom
  (params (Key :type Key%20Structure :default "None"))
  ;[1 1 1] Change VR Smart Phone's display's material  when  took a photo.  It will display [Photo_ShowOutTime] seconds and change back to live mode.
  (:Pressed
    (if (== (Variables|Default|GetSmartPhoneMode) 0)
      (if (Variables|/Script/hukuokaGame.PlayerCharacter|Getvr_InCameraMode (Variables|Default|Getplayer1))
        _
        (else
          _))
      (Rendering|ClearRenderTarget2D "/Game/Materials/photoTarget.photoTarget" "(R=0.000000,G=0.000000,B=0.000000,A=255.000000)")
      (Rendering|DrawMaterialtoRenderTarget "/Game/Materials/photoTarget.photoTarget" "/Game/Materials/smartPhoneDisplay.SmartPhoneDisplay")
      (Variables|Default|SetisShowingPhoto true)
      (CallFunction|SetCameraUIONOFF (Variables|Default|GetVRSmartPhoneUI) false)
      (Rendering|Material|SetMaterial (Variables|Default|GetVRSmartPhoneDisplay) 0 "/Game/Materials/PhotoDisplay.PhotoDisplay")
      (Utilities|FlowControl|Delay (Variables|Default|GetPhoto_ShowOutTime))
      (Rendering|Material|SetMaterial (Variables|Default|GetVRSmartPhoneDisplay) 0 "/Game/Materials/smartPhoneDisplay.SmartPhoneDisplay")
      (Variables|Default|SetisShowingPhoto false)
      (CallFunction|SetCameraUIONOFF (Variables|Default|GetVRSmartPhoneUI) true))))

(event Input|KeyboardEvents|NumPadFour
  (params (Key :type Key%20Structure :default "None"))
  (bind _camerafov_default (Variables|Default|GetCameraFOV_default))
  (:Pressed
    (switch int (Variables|Default|GetSmartPhoneMode)
      (:0
        (Variables|Default|SetSmartPhoneMode 3)
        (Class|WidgetSwitcher|SetActiveWidgetIndex (Variables|/Game/UI/VRsmartPhoneWidget.VRsmartPhoneWidget_C|GetDisplaySwitcher (Variables|Default|GetVRSmartPhoneUI)) 4)
        (CallFunction|HeartBeatStatusSwitch))
      (:1
        (Variables|Default|SetSmartPhoneMode 0)
        (Class|WidgetSwitcher|SetActiveWidgetIndex (Variables|/Game/UI/VRsmartPhoneWidget.VRsmartPhoneWidget_C|GetDisplaySwitcher (Variables|Default|GetVRSmartPhoneUI)))
        (Variables|/Script/Engine.SceneCaptureComponent2D|SetFOVAngle (Variables|Default|GetVRSmartPhoneCamera) _camerafov_default)
        (Variables|Default|SetCameraFOV_Current _camerafov_default)
        (Variables|Default|SetHeartBeat_isAppOn false))
      (:2
        (Variables|Default|SetSmartPhoneMode 1)
        (if (Variables|Default|GetCameraLightOn)
          (CallFunction|SetLightUIONOFF true)
          (else
            (CallFunction|SetLightUIONOFF false)))
        (Class|WidgetSwitcher|SetActiveWidgetIndex (Variables|/Game/UI/VRsmartPhoneWidget.VRsmartPhoneWidget_C|GetDisplaySwitcher (Variables|Default|GetVRSmartPhoneUI)) 1))
      (:3
        (Variables|Default|SetSmartPhoneMode 2)
        (Variables|Default|SetHeartBeat_isAppOn false)
        (CallFunction|SetMissionContentsSingle)
        (if (Class|HeadMountedDisplayFunctionLibrary|IsHeadMountedDisplayEnabled)
          (Class|WidgetSwitcher|SetActiveWidgetIndex (Variables|/Game/UI/VRsmartPhoneWidget.VRsmartPhoneWidget_C|GetDisplaySwitcher (Variables|Default|GetVRSmartPhoneUI)) 2)
          (else
            (Class|WidgetSwitcher|SetActiveWidgetIndex (Variables|/Game/UI/VRsmartPhoneWidget.VRsmartPhoneWidget_C|GetDisplaySwitcher (Variables|Default|GetVRSmartPhoneUI)) 3)))))))

(event Input|KeyboardEvents|A
  (params (Key :type Key%20Structure :default "None"))
  ;[1 1 1] HeartBeatアプリのOn/Off　 by_朱
)

(event Input|GamepadEvents|GamepadFaceButtonBottom
  (params (Key :type Key%20Structure :default "None"))
  ;[1 1 1] VRのスマホライトOn/Off  / Change VR Smart Phone Camera Light on/off
  (:Pressed
    (if (== (Variables|Default|GetSmartPhoneMode) 1)
      (if (Variables|Default|GetCameraLightOn)
        (Rendering|SetVisibility (Variables|Default|GetCameraLight) false false)
        (Rendering|SetVisibility (Variables|Default|GetCameraLight2) false false)
        (Variables|Default|SetCameraLightOn false)
        (CallFunction|SetLightUIONOFF false)
        (else
          (Rendering|SetVisibility (Variables|Default|GetCameraLight) true false)
          (Rendering|SetVisibility (Variables|Default|GetCameraLight2) true false)
          (Variables|Default|SetCameraLightOn true)
          (CallFunction|SetLightUIONOFF true))))))

(event Input|KeyboardEvents|B
  (params (Key :type Key%20Structure :default "None"))
  (bind _camerafov_default (Variables|Default|GetCameraFOV_default))
  (:Pressed
    (switch int (Variables|Default|GetSmartPhoneMode)
      (:0
        (Variables|Default|SetSmartPhoneMode 1)
        (if (Variables|Default|GetCameraLightOn)
          (CallFunction|SetLightUIONOFF true)
          (else
            (CallFunction|SetLightUIONOFF false)))
        (Class|WidgetSwitcher|SetActiveWidgetIndex (Variables|/Game/UI/VRsmartPhoneWidget.VRsmartPhoneWidget_C|GetDisplaySwitcher (Variables|Default|GetVRSmartPhoneUI)) 1))
      (:1
        (Variables|Default|SetSmartPhoneMode 2)
        (CallFunction|SetMissionContentsSingle)
        (if (Class|HeadMountedDisplayFunctionLibrary|IsHeadMountedDisplayEnabled)
          (Class|WidgetSwitcher|SetActiveWidgetIndex (Variables|/Game/UI/VRsmartPhoneWidget.VRsmartPhoneWidget_C|GetDisplaySwitcher (Variables|Default|GetVRSmartPhoneUI)) 2)
          (else
            (Class|WidgetSwitcher|SetActiveWidgetIndex (Variables|/Game/UI/VRsmartPhoneWidget.VRsmartPhoneWidget_C|GetDisplaySwitcher (Variables|Default|GetVRSmartPhoneUI)) 3))))
      (:2
        (Variables|Default|SetSmartPhoneMode 3)
        (Class|WidgetSwitcher|SetActiveWidgetIndex (Variables|/Game/UI/VRsmartPhoneWidget.VRsmartPhoneWidget_C|GetDisplaySwitcher (Variables|Default|GetVRSmartPhoneUI)) 4)
        (CallFunction|HeartBeatStatusSwitch))
      (:3
        (Variables|Default|SetSmartPhoneMode 0)
        (Class|WidgetSwitcher|SetActiveWidgetIndex (Variables|/Game/UI/VRsmartPhoneWidget.VRsmartPhoneWidget_C|GetDisplaySwitcher (Variables|Default|GetVRSmartPhoneUI)))
        (Variables|/Script/Engine.SceneCaptureComponent2D|SetFOVAngle (Variables|Default|GetVRSmartPhoneCamera) _camerafov_default)
        (Variables|Default|SetCameraFOV_Current _camerafov_default)
        (Variables|Default|SetHeartBeat_isAppOn false)))))

(event Input|KeyboardEvents|Add
  (params (Key :type Key%20Structure :default "None"))
  ;[1 1 1] CameraZoom
  (:Pressed
    (if (== (Variables|Default|GetSmartPhoneMode) 0)
      (CallFunction|CameraZoom true))))

(event Input|KeyboardEvents|Z
  (params (Key :type Key%20Structure :default "None"))
  ;[1 1 1] Change VR Smart Phone's display's material  when  took a photo.  It will display [Photo_ShowOutTime] seconds and change back to live mode.
  (:Pressed
    (if (== (Variables|Default|GetSmartPhoneMode) 0)
      (if (Variables|/Script/hukuokaGame.PlayerCharacter|Getvr_InCameraMode (Variables|Default|Getplayer1))
        _
        (else
          _))
      (Rendering|ClearRenderTarget2D "/Game/Materials/photoTarget.photoTarget" "(R=0.000000,G=0.000000,B=0.000000,A=255.000000)")
      (Rendering|DrawMaterialtoRenderTarget "/Game/Materials/photoTarget.photoTarget" "/Game/Materials/smartPhoneDisplay.SmartPhoneDisplay")
      (Variables|Default|SetisShowingPhoto true)
      (CallFunction|SetCameraUIONOFF (Variables|Default|GetVRSmartPhoneUI) false)
      (Rendering|Material|SetMaterial (Variables|Default|GetVRSmartPhoneDisplay) 0 "/Game/Materials/PhotoDisplay.PhotoDisplay")
      (Utilities|FlowControl|Delay (Variables|Default|GetPhoto_ShowOutTime))
      (Rendering|Material|SetMaterial (Variables|Default|GetVRSmartPhoneDisplay) 0 "/Game/Materials/smartPhoneDisplay.SmartPhoneDisplay")
      (Variables|Default|SetisShowingPhoto false)
      (CallFunction|SetCameraUIONOFF (Variables|Default|GetVRSmartPhoneUI) true))))

(event Input|KeyboardEvents|X
  (params (Key :type Key%20Structure :default "None"))
  ;[1 1 1] VRのスマホライトOn/Off  / Change VR Smart Phone Camera Light on/off
  (:Pressed
    (if (== (Variables|Default|GetSmartPhoneMode) 1)
      (if (Variables|Default|GetCameraLightOn)
        (Rendering|SetVisibility (Variables|Default|GetCameraLight) false false)
        (Rendering|SetVisibility (Variables|Default|GetCameraLight2) false false)
        (Variables|Default|SetCameraLightOn false)
        (CallFunction|SetLightUIONOFF false)
        (else
          (Rendering|SetVisibility (Variables|Default|GetCameraLight) true false)
          (Rendering|SetVisibility (Variables|Default|GetCameraLight2) true false)
          (Variables|Default|SetCameraLightOn true)
          (CallFunction|SetLightUIONOFF true))))))

(event Input|KeyboardEvents|Subtract
  (params (Key :type Key%20Structure :default "None"))
  ;[1 1 1] CameraZoom
  (:Pressed
    (if (== (Variables|Default|GetSmartPhoneMode) 0)
      (CallFunction|CameraZoom false))))

(event Input|GamepadEvents|GamepadRightTrigger
  (params (Key :type Key%20Structure :default "None"))
  (bind _camerafov_default (Variables|Default|GetCameraFOV_default))
  (:Pressed
    (switch int (Variables|Default|GetSmartPhoneMode)
      (:0
        (Variables|Default|SetSmartPhoneMode 1)
        (if (Variables|Default|GetCameraLightOn)
          (CallFunction|SetLightUIONOFF true)
          (else
            (CallFunction|SetLightUIONOFF false)))
        (Class|WidgetSwitcher|SetActiveWidgetIndex (Variables|/Game/UI/VRsmartPhoneWidget.VRsmartPhoneWidget_C|GetDisplaySwitcher (Variables|Default|GetVRSmartPhoneUI)) 1))
      (:1
        (Variables|Default|SetSmartPhoneMode 2)
        (CallFunction|SetMissionContentsSingle)
        (if (Class|HeadMountedDisplayFunctionLibrary|IsHeadMountedDisplayEnabled)
          (Class|WidgetSwitcher|SetActiveWidgetIndex (Variables|/Game/UI/VRsmartPhoneWidget.VRsmartPhoneWidget_C|GetDisplaySwitcher (Variables|Default|GetVRSmartPhoneUI)) 2)
          (else
            (Class|WidgetSwitcher|SetActiveWidgetIndex (Variables|/Game/UI/VRsmartPhoneWidget.VRsmartPhoneWidget_C|GetDisplaySwitcher (Variables|Default|GetVRSmartPhoneUI)) 3))))
      (:2
        (Variables|Default|SetSmartPhoneMode 3)
        (Class|WidgetSwitcher|SetActiveWidgetIndex (Variables|/Game/UI/VRsmartPhoneWidget.VRsmartPhoneWidget_C|GetDisplaySwitcher (Variables|Default|GetVRSmartPhoneUI)) 4)
        (CallFunction|HeartBeatStatusSwitch))
      (:3
        (Variables|Default|SetSmartPhoneMode 0)
        (Class|WidgetSwitcher|SetActiveWidgetIndex (Variables|/Game/UI/VRsmartPhoneWidget.VRsmartPhoneWidget_C|GetDisplaySwitcher (Variables|Default|GetVRSmartPhoneUI)))
        (Variables|/Script/Engine.SceneCaptureComponent2D|SetFOVAngle (Variables|Default|GetVRSmartPhoneCamera) _camerafov_default)
        (Variables|Default|SetCameraFOV_Current _camerafov_default)
        (Variables|Default|SetHeartBeat_isAppOn false)))))

(fn ConstructionScript)

(fn ChangetoCamera
  (params (Mode :type Integer))
  (Rendering|Material|SetMaterial (Variables|Default|GetVRSmartPhoneDisplay) 0 "/Game/Materials/App_Icon_Camera.App_Icon_Camera"))

(fn SetCameraUIONOFF
  (params (VRSmartPhoneUI :type V%20Rsmart%20Phone%20Widget%20Object%20Reference) (UI_isON :type Boolean))
  (if UI_isON
    (Widget|SetVisibility (Variables|/Game/UI/VRsmartPhoneWidget.VRsmartPhoneWidget_C|GetAiming_Bottom VRSmartPhoneUI) "Visible")
    (Widget|SetVisibility (Variables|/Game/UI/VRsmartPhoneWidget.VRsmartPhoneWidget_C|GetAiming_Center VRSmartPhoneUI) "Visible")
    (Widget|SetVisibility (Variables|/Game/UI/VRsmartPhoneWidget.VRsmartPhoneWidget_C|GetAiming_Top VRSmartPhoneUI) "Visible")
    (else
      (Widget|SetVisibility (Variables|/Game/UI/VRsmartPhoneWidget.VRsmartPhoneWidget_C|GetAiming_Bottom VRSmartPhoneUI) "Hidden")
      (Widget|SetVisibility (Variables|/Game/UI/VRsmartPhoneWidget.VRsmartPhoneWidget_C|GetAiming_Center VRSmartPhoneUI) "Hidden")
      (Widget|SetVisibility (Variables|/Game/UI/VRsmartPhoneWidget.VRsmartPhoneWidget_C|GetAiming_Top VRSmartPhoneUI) "Hidden"))))

(fn SetLightUIONOFF
  (params (Light_isOn :type Boolean))
  (bind _vrsmartphoneui (Variables|Default|GetVRSmartPhoneUI))
  (bind _vrsmartphoneui_2 (Variables|Default|GetVRSmartPhoneUI))
  (bind _light_off (Variables|/Game/UI/VRsmartPhoneWidget.VRsmartPhoneWidget_C|GetLight_Off _vrsmartphoneui_2))
  (bind _light_on (Variables|/Game/UI/VRsmartPhoneWidget.VRsmartPhoneWidget_C|GetLight_On _vrsmartphoneui))
  (if Light_isOn
    (Widget|SetVisibility (Variables|/Game/UI/VRsmartPhoneWidget.VRsmartPhoneWidget_C|GetLight_Off (Variables|Default|GetVRSmartPhoneUI)) "Hidden")
    (Widget|SetVisibility _light_on "Visible")
    (Class|Image|SetOpacity (Variables|/Game/UI/VRsmartPhoneWidget.VRsmartPhoneWidget_C|GetLight_Off (Variables|Default|GetVRSmartPhoneUI)) 1.0)
    (Class|Image|SetOpacity (Variables|/Game/UI/VRsmartPhoneWidget.VRsmartPhoneWidget_C|GetLight_On (Variables|Default|GetVRSmartPhoneUI)) 1.0)
    (Variables|Default|SetdisAppearingImage _light_on)
    (else
      (Widget|SetVisibility _light_off "Visible")
      (Widget|SetVisibility (Variables|/Game/UI/VRsmartPhoneWidget.VRsmartPhoneWidget_C|GetLight_On (Variables|Default|GetVRSmartPhoneUI)) "Hidden")
      (Class|Image|SetOpacity (Variables|/Game/UI/VRsmartPhoneWidget.VRsmartPhoneWidget_C|GetLight_On (Variables|Default|GetVRSmartPhoneUI)) 1.0)
      (Class|Image|SetOpacity (Variables|/Game/UI/VRsmartPhoneWidget.VRsmartPhoneWidget_C|GetLight_Off (Variables|Default|GetVRSmartPhoneUI)) 1.0)
      (Variables|Default|SetdisAppearingImage _light_off))))

(fn SetMissionContentsSingle
  (bind _player1 (Variables|Default|Getplayer1))
  (bind _vr_smartphone_mission_num (Variables|/Script/hukuokaGame.PlayerCharacter|Getvr_SmartPhone_Mission_Num _player1))
  (bind _returnvalue (Utilities|String|ToString(Integer) _vr_smartphone_mission_num))
  (bind _returnvalue_2 (Utilities|String|StringToName _returnvalue))
  (bind _returnvalue_3 (Utilities|GetDataTableRow "/Game/UI/mission_List.mission_List" _returnvalue_2)
    (:then
      (Rendering|Components|TextRender|SetText (Variables|/Game/UI/VRsmartPhoneWidget.VRsmartPhoneWidget_C|GetMissionContentsBox (Variables|Default|GetVRSmartPhoneUI)) (Utilities|Text|ToText(String) (.MissionContents (Utilities|Struct|BreakMissions_Struct _returnvalue_3))))
      (Rendering|Components|TextRender|SetText (Variables|/Game/UI/VRsmartPhoneWidget.VRsmartPhoneWidget_C|GetMissionContentsBox_Straight (Variables|Default|GetVRSmartPhoneUI)) (Utilities|Text|ToText(String) (.MissionContents (Utilities|Struct|BreakMissions_Struct _returnvalue_3))))
      (Development|PrintString (Utilities|String|ToString(Name) _returnvalue_2) true true "(R=1.000000,G=0.229310,B=0.825617,A=1.000000)" 0.01))))

(fn SetMissionContentsMulti
  (bind _player1 (Variables|Default|Getplayer1))
  (bind _vr_smartphone_mission_num (Variables|/Script/hukuokaGame.PlayerCharacter|Getvr_SmartPhone_Mission_Num _player1))
  (bind _returnvalue (Utilities|String|ToString(Integer) _vr_smartphone_mission_num))
  (bind _returnvalue_2 (Utilities|String|StringToName _returnvalue))
  (bind _returnvalue_3 (Utilities|GetDataTableRow "/Game/UI/mission_List.mission_List" _returnvalue_2)
    (:then
      (Rendering|Components|TextRender|SetText (Variables|/Game/UI/VRsmartPhoneWidget.VRsmartPhoneWidget_C|GetMissionContentsBox (Variables|Default|GetVRSmartPhoneUI)) (Utilities|Text|ToText(String) (.MissionContents (Utilities|Struct|BreakMissions_Struct _returnvalue_3))))
      (Development|PrintString (Utilities|String|ToString(Name) _returnvalue_2) true true "(R=1.000000,G=0.229310,B=0.825617,A=1.000000)" 0.01))))

(fn UIDisappearingFunc
  (params (deltaTime :type Float%20%28single-precision%29) (Image :type Image%20Object%20Reference))
  (bind _returnvalue (* deltaTime 0.25))
  (bind _colorandopacity (Variables|/Script/UMG.Image|GetColorAndOpacity Image))
  (bind _returnvalue_2 (- (.a _colorandopacity) _returnvalue))
  (bind _output_get (Variables|Default|SetLightUI_CountingTime (+ deltaTime (Variables|Default|GetLightUI_CountingTime))))
  (Math|Float|CompareFloat _output_get (Variables|Default|GetLightUI_AppearingTime)
    (:>
      _)
    (:==
      _))
  (if (<= _returnvalue_2 0.0)
    (Class|Image|SetOpacity Image 0.0)
    (Variables|Default|SetLighyUI_isShowing false)
    (Variables|Default|SetLightUI_CountingTime 0.0)
    (else
      (Class|Image|SetOpacity Image _returnvalue_2))))

(fn CameraZoom
  (params (isZoomIn :type Boolean))
  (bind _vrsmartphonecamera (Variables|Default|GetVRSmartPhoneCamera))
  (if isZoomIn
    (if (> (Variables|Default|GetCameraFOV_Current) 6e+01)
      (Variables|/Script/Engine.SceneCaptureComponent2D|SetFOVAngle _vrsmartphonecamera (- (Variables|Default|GetCameraFOV_Current) 5.0))
      (Variables|Default|SetCameraFOV_Current (- (Variables|Default|GetCameraFOV_Current) 5.0)))
    (elif (< (Variables|Default|GetCameraFOV_Current) (Variables|Default|GetCameraFOV_default))
      (Variables|/Script/Engine.SceneCaptureComponent2D|SetFOVAngle _vrsmartphonecamera (+ (Variables|Default|GetCameraFOV_Current) 5.0))
      (Variables|Default|SetCameraFOV_Current (+ (Variables|Default|GetCameraFOV_Current) 5.0)))))

(fn HeartBeatStatusSwitch
  (bind _vrsmartphoneui (Variables|Default|GetVRSmartPhoneUI))
  (if (Variables|Default|GetHeartBeat_isAppOn)
    (Default|HeartBeatOff _vrsmartphoneui)
    (else
      (Default|HeartBeaton _vrsmartphoneui)))
  (Variables|Default|SetHeartBeat_isAppOn (not (Variables|Default|GetHeartBeat_isAppOn))))

(fn GetPlayertoEnemyAngle)