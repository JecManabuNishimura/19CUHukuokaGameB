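; BP_Beaker is a destructible glass beaker that the player can knock over to make a noise that an enemy AI is told about.
; A box overlap by an actor tagged Player applies an impulse to the destructible component.
; The first hit on a component tagged Floor plays a glass-break sound and calls MakedNoisePawn on a referenced BP_AI_Enemy, passing the beaker itself.
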(event OnComponentBeginOverlap(BoxColision)
  (params (OverlappedComponent :type Primitive%20Component%20Object%20Reference) (OtherActor :type Actor%20Object%20Reference) (OtherComp :type Primitive%20Component%20Object%20Reference) (OtherBodyIndex :type Integer) (bFromSweep :type Boolean) (SweepResult :type Hit%20Result%20Structure%20%28by%20ref%29))
  ;[1 1 1] Playerがぶつかった時の処理
  (if (Actor|ActorHasTag OtherActor "Player")
    (Physics|AddImpulse (Variables|Default|GetDestructibleComponent) (Variables|Default|GetImpulseValue) "None" false)))

(event OnComponentHit(DestructibleComponent)
  (params (HitComponent :type Primitive%20Component%20Object%20Reference) (OtherActor :type Actor%20Object%20Reference) (OtherComp :type Primitive%20Component%20Object%20Reference) (NormalImpulse :type Vector :default "0, 0, 0") (Hit :type Hit%20Result%20Structure%20%28by%20ref%29))
  (if (Components|ComponentHasTag OtherComp "Floor")
    (Utilities|FlowControl|DoOnce false
      (:Completed
        (Audio|PlaySoundatLocation "/Game/SE/Glass_Break.Glass_Break" (Transformation|GetActorLocation) "0, 0, 0" 1.0 1.0 0.0 0 0 0)
        (Default|MakedNoisePawn (.AsBP%20AI%20Enemy (Utilities|Casting|CastToBP_AI_Enemy (Variables|Default|GetNewVar_0))) self)))))

(event EventBeginPlay)

(event Collision|EventActorBeginOverlap
  (params (OtherActor :type Actor%20Object%20Reference)))

(event EventTick
  (params (DeltaSeconds :type Float%20%28single-precision%29)))

(event Collision|EventHit
  (params (MyComp :type Primitive%20Component%20Object%20Reference) (Other :type Actor%20Object%20Reference) (OtherComp :type Primitive%20Component%20Object%20Reference) (bSelfMoved :type Boolean) (HitLocation :type Vector :default "0, 0, 0") (HitNormal :type Vector :default "0, 0, 0") (NormalImpulse :type Vector :default "0, 0, 0") (Hit :type Hit%20Result%20Structure%20%28by%20ref%29)))

(fn ConstructionScript)