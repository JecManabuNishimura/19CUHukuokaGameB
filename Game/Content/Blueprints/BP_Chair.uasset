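; BP_Chair is a chair actor that plays a scrape sound when the player shoves it.
; On a ChairMesh hit from a Player-tagged actor, it stores its location, waits briefly, then checks whether it moved past a small threshold on X or Y.
; A DoOnce gate, reset after a short delay, keeps repeated hits from stacking the sound.
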(event OnComponentHit(ChairMesh)
  (params (HitComponent :type Primitive%20Component%20Object%20Reference) (OtherActor :type Actor%20Object%20Reference) (OtherComp :type Primitive%20Component%20Object%20Reference) (NormalImpulse :type Vector :default "0, 0, 0") (Hit :type Hit%20Result%20Structure%20%28by%20ref%29))
  (bind _returnvalue (Transformation|GetActorLocation))
  (if (Actor|ActorHasTag OtherActor "Player")
    (Variables|Default|SetPrev_Loc (Transformation|GetActorLocation))
    (Utilities|FlowControl|Delay 0.05)
    (if (or (> (Math|Float|Absolute(Float) (.x (- (Variables|Default|GetPrev_Loc) _returnvalue))) 3.0) (> (Math|Float|Absolute(Float) (.y (- (Variables|Default|GetPrev_Loc) _returnvalue))) 3.0))
      (Utilities|FlowControl|DoOnce false :!label _label
        (:Completed
          (Audio|PlaySoundatLocation "/Game/SE/Chair_Move_New.Chair_Move_New" _returnvalue "0, 0, 0" 0.5 1.0 0.0 0 0 0)
          (Utilities|FlowControl|Delay 0.4)
          (goto _label Reset))))))

(event EventBeginPlay)

(event Collision|EventActorBeginOverlap
  (params (OtherActor :type Actor%20Object%20Reference)))

(event EventTick
  (params (DeltaSeconds :type Float%20%28single-precision%29)))

(fn ConstructionScript)