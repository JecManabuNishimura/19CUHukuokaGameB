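; PhotoAlbum is an in-game album actor that displays two saved images on its Photo1 and Photo2 components.
; BeginPlay gives each component its own dynamic instance of the Album_PhotoDisplay material.
; The ShowPhoto1 and ShowPhoto2 events each run once, importing ss1.png or ss2.png from the project's img folder at runtime into that material's PhotoTarget texture parameter.
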(event Custom|ShowPhoto1
  (Utilities|FlowControl|DoOnce false
    (:Completed
      (bind _returnvalue (Class|KismetRenderingLibrary|ImportFileasTexture2D (Utilities|String|Append (Class|KismetSystemLibrary|GetProjectDirectory) "img/ss1.png")))
      (Rendering|Material|SetTextureParameterValue (Variables|Default|GetDynamicMat) "PhotoTarget" _returnvalue))))

(event Custom|ShowPhoto2
  (Utilities|FlowControl|DoOnce false
    (:Completed
      (bind _returnvalue (Class|KismetRenderingLibrary|ImportFileasTexture2D (Utilities|String|Append (Class|KismetSystemLibrary|GetProjectDirectory) "img/ss2.png")))
      (Rendering|Material|SetTextureParameterValue (Variables|Default|GetDynamicMat2) "PhotoTarget" _returnvalue))))

(event EventBeginPlay
  (bind _returnvalue (Rendering|Material|CreateDynamicMaterialInstance (Variables|Default|GetPhoto1) 0 "/Game/Materials/Album_PhotoDisplay.Album_PhotoDisplay" "None" :!class /Script/Engine.PrimitiveComponent))
  (Variables|Default|SetDynamicMat _returnvalue)
  (Rendering|Material|SetMaterial (Variables|Default|GetPhoto1) 0 (Variables|Default|GetDynamicMat))
  (bind _returnvalue_2 (Rendering|Material|CreateDynamicMaterialInstance (Variables|Default|GetPhoto2) 0 "/Game/Materials/Album_PhotoDisplay.Album_PhotoDisplay" "None" :!class /Script/Engine.PrimitiveComponent))
  (Variables|Default|SetDynamicMat2 _returnvalue_2)
  (Rendering|Material|SetMaterial (Variables|Default|GetPhoto2) 0 (Variables|Default|GetDynamicMat2)))

(event Collision|EventActorBeginOverlap
  (params (OtherActor :type Actor%20Object%20Reference)))

(event EventTick
  (params (DeltaSeconds :type Float%20%28single-precision%29)))

(fn ConstructionScript)