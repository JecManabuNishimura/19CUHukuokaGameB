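; Baby actor that acts as a one-shot noise trap, crying when the player moves too fast near it.
; Box overlaps with Player-tagged actors set an in-range flag, and Tick compares the player's speed against a threshold while that flag is set.
; Crying launches the referenced Enemy into its hearing state at the baby's location, notifies a DestroyDoor and plays a sound.
; An unconnected BP_AI_Enemy alert branch remains unused.
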(event OnComponentBeginOverlap(Boxcol)
  (params (OverlappedComponent :type Primitive%20Component%20Object%20Reference) (OtherActor :type Actor%20Object%20Reference) (OtherComp :type Primitive%20Component%20Object%20Reference) (OtherBodyIndex :type Integer) (bFromSweep :type Boolean) (SweepResult :type Hit%20Result%20Structure%20%28by%20ref%29))
  (if (Actor|ActorHasTag OtherActor "Player")
    (Variables|Default|SetisPlayerInCryRange true)))

(event OnComponentEndOverlap(Boxcol)
  (params (OverlappedComponent :type Primitive%20Component%20Object%20Reference) (OtherActor :type Actor%20Object%20Reference) (OtherComp :type Primitive%20Component%20Object%20Reference) (OtherBodyIndex :type Integer))
  (if (Actor|ActorHasTag OtherActor "Player")
    (Variables|Default|SetisPlayerInCryRange false)))

(event EventBeginPlay
  (Variables|Default|SetPlayer (Game|GetPlayerCharacter 0)))

(event EventTick
  (params (DeltaSeconds :type Float%20%28single-precision%29))
  ;[1 1 1] Playerがぶつかった時の処理
  (if (not (Variables|Default|GetisCry))
    (if (Variables|Default|GetisPlayerInCryRange)
      (if (> (Math|Vector|VectorLength (Variables|/Script/Engine.MovementComponent|GetVelocity (Pawn|GetMovementComponent (Variables|/Script/Engine.Actor|GetInstigator (Variables|Default|GetPlayer))))) (Variables|Default|GetcrySpped))
        (Variables|Default|SetisCry true)
        (bind _asenemy (Utilities|Casting|CastToEnemy (Variables|Default|GetEnemy)))
        (Variables|/Script/hukuokaGame.Enemy|Setis_launch_ _asenemy true)
        (Class|Enemy|SetHearPos _asenemy (Transformation|GetActorLocation))
        (Variables|/Script/hukuokaGame.Enemy|Setenemy_state_ _asenemy "kHear")
        (Development|PrintString "Baby is crying" true true "(R=0.000000,G=0.660000,B=1.000000,A=1.000000)" 5.0)
        (bind _asdestroy_door (Utilities|Casting|CastToDestroyDoor (Variables|Default|GetDoor)))
        (Class|DestroyDoor|GetIsCry _asdestroy_door true)
        (Audio|PlaySoundatLocation 0 (Transformation|GetActorLocation) "0, 0, 0" 1.0 1.0 0.0 0 0 0)))))

(fn ConstructionScript)