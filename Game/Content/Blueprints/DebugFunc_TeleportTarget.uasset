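; Debug actor that lets the player teleport to preset target actors or return to the Title level.
; BeginPlay enables input, caches the player character and creates the debug menu widget, which Tab shows or hides along with debug mode.
; In debug mode, the TeleportDebug key's display name becomes an array index: zero opens Title, while valid entries move the player to that target's location and rotation, then close the menu.
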(event EventBeginPlay
  (bind _returnvalue (Game|GetPlayerController 0))
  (Variables|Default|SetplayerController _returnvalue)
  (Input|EnableInput _returnvalue)
  (while (not (Utilities|IsValid (Variables|Default|GetplayerCharacter)))
    (Variables|Default|SetplayerCharacter (Game|GetPlayerCharacter 0))
    (bind _returnvalue_2 (UserInterface|CreateWidget "/Game/UI/DebugMenu.DebugMenu_C"))
    (Variables|Default|SetdebugMenuUI _returnvalue_2)))

(event Collision|EventActorBeginOverlap
  (params (OtherActor :type Actor%20Object%20Reference)))

(event EventTick
  (params (DeltaSeconds :type Float%20%28single-precision%29)))

(event Input|ActionEvents|InputActionTeleportDebug
  (params (Key :type Key%20Structure :default "None"))
  (bind _returnvalue (Class|KismetInputLibrary|KeyGetDisplayName Key))
  (bind _playercharacter (Variables|Default|GetplayerCharacter))
  (bind _newvar_1 (Variables|Default|GetNewVar_1))
  (bind _returnvalue_2 (Utilities|String|ToString(Text) _returnvalue))
  (bind _returnvalue_3 (Math|Conversions|ToInteger(Byte) _returnvalue_2))
  (bind _output (Utilities|Array|Get(acopy) _newvar_1 _returnvalue_3))
  (bind _returnvalue_4 (Transformation|GetActorTransform _output))
  (:Pressed
    (if (Variables|Default|GetisDebugMode)
      (if (== _returnvalue_3 0)
        (Game|OpenLevel(byName) "Title")
        (else
          (Utilities|IsValid _output
            (:Is%20Valid
              (Transformation|SetActorTransform _playercharacter (Math|Transform|MakeTransform (.location _returnvalue_4) (.rotation _returnvalue_4) (Transformation|GetActorScale3D _playercharacter)))
              (Variables|Default|SetisDebugMode false)
              (Widget|RemovefromParent (Variables|Default|GetdebugMenuUI)))))))))

(event Input|KeyboardEvents|Tab
  (params (Key :type Key%20Structure :default "None"))
  (bind _debugmenuui (Variables|Default|GetdebugMenuUI))
  (:Pressed
    (bind _output_get (Variables|Default|SetisDebugMode (not (Variables|Default|GetisDebugMode))))
    (if _output_get
      (UserInterface|Viewport|AddtoViewport _debugmenuui 0)
      (else
        (Widget|RemovefromParent _debugmenuui)))))

(fn ConstructionScript)