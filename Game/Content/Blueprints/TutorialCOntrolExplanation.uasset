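; Tutorial trigger actor that shows a control-explanation widget once when the player overlaps its box, then destroys itself.
; With a headset enabled, it spawns a scaled-down BP_VR_ControlManual, attaches it to the player's camera at an offset and passes it the configured widget with a limited lifetime.
; Without VR, it adds the same widget class straight to the viewport.
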(event OnComponentBeginOverlap(Box)
  (params (OverlappedComponent :type Primitive%20Component%20Object%20Reference) (OtherActor :type Actor%20Object%20Reference) (OtherComp :type Primitive%20Component%20Object%20Reference) (OtherBodyIndex :type Integer) (bFromSweep :type Boolean) (SweepResult :type Hit%20Result%20Structure%20%28by%20ref%29))
  (if (Actor|ActorHasTag OtherActor "Player")
    (Utilities|FlowControl|DoOnce false
      (:Completed
        (if (Class|HeadMountedDisplayFunctionLibrary|IsHeadMountedDisplayEnabled)
          ;[1 1 1] Generate VR Dialogue
          (bind _asbp_player_character (Utilities|Casting|CastToBP_PlayerCharacter (Game|GetPlayerCharacter 0)))
          (bind _output_get (Variables|Default|SetPlayer1 _asbp_player_character))
          (bind _returnvalue (Game|SpawnActorfromClass "/Game/Blueprints/BP_VR_ControlManual.BP_VR_ControlManual_C" (Math|Transform|MakeTransform (Transformation|GetActorLocation _output_get) "0,180.000000, 0" "0.200000,0.200000,0.200000") "Undefined" 0 0))
          (bind _output_get_2 (Variables|Default|SetVRManualWidgetActor _returnvalue))
          (Transformation|AttachComponentToComponent _output_get_2 (Variables|/Script/hukuokaGame.PlayerCharacter|Getm_pCamera (Variables|Default|GetPlayer1)) "None" "KeepRelative" "KeepRelative" "KeepRelative" true)
          (Default|ChangeWidget (Variables|Default|GetVRManualWidgetActor) (Variables|Default|GetGenerateWidget) 7.0)
          (Transformation|SetActorRelativeLocation (Variables|Default|GetVRManualWidgetActor) "250.000000,-120.000000,-100.000000")
          (Actor|DestroyActor)
          (else
            (bind _returnvalue_2 (UserInterface|CreateWidget (Variables|Default|GetGenerateWidget)))
            (UserInterface|Viewport|AddtoViewport _returnvalue_2 0)
            (Actor|DestroyActor)))))))

(event EventBeginPlay)

(event Collision|EventActorBeginOverlap
  (params (OtherActor :type Actor%20Object%20Reference)))

(event EventTick
  (params (DeltaSeconds :type Float%20%28single-precision%29)))

(fn ConstructionScript)