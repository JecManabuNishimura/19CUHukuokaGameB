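; Test actor that plays an attenuated enemy footstep cue at its own location every half second, using a timer accumulated in Tick.
; A disconnected branch sketches sound occlusion: a multi line trace toward the player lowers Volume per hit, zeroing it for actors tagged as complete sound insulation.
; That branch never runs, and Volume is not passed to the sound.
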(event EventBeginPlay
  (Variables|Default|Setplayer_character (Game|GetPlayerCharacter 0)))

(event Collision|EventActorBeginOverlap
  (params (OtherActor :type Actor%20Object%20Reference)))

(event EventTick
  (params (DeltaSeconds :type Float%20%28single-precision%29))
  (bind _output_get (Variables|Default|Settime_count (+ DeltaSeconds (Variables|Default|Gettime_count))))
  (if (>= _output_get 0.5)
    (Variables|Default|Settime_count 0.0)
    (Variables|Default|Setvolume 1.0)
    (Audio|PlaySoundatLocation "/Game/SE/Enemy_Footstep_Cue.Enemy_Footstep_Cue" (Transformation|GetActorLocation) "0, 0, 0" 1.0 1.0 0.0 "/Game/SE/Base_Attenuation.Base_Attenuation" 0 0)))

(fn ConstructionScript)