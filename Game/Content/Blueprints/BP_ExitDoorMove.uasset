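; Exit door actor with two sliding panels that a Player-tagged actor can open once every MissionMap entry is true.
; Trigger overlap plays the OpenDoor timeline if IsSwitchOn is set, otherwise it only sets that flag; the lever loop reads no lever state.
; Tick checks every three seconds while open, reversing the timeline to close once the overlap flag is clear.
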(event OnComponentBeginOverlap(m_pEventTriggerBox)
  (params (OverlappedComponent :type Primitive%20Component%20Object%20Reference) (OtherActor :type Actor%20Object%20Reference) (OtherComp :type Primitive%20Component%20Object%20Reference) (OtherBodyIndex :type Integer) (bFromSweep :type Boolean) (SweepResult :type Hit%20Result%20Structure%20%28by%20ref%29))
  ;[1 1 1] プレイヤーを検知したら開くフラグおよび検知フラグを立てる
  (bind _ismissionclear (CallFunction|IsMissionClear))
  (if _ismissionclear
    (if (Actor|ActorHasTag OtherActor "Player")
      (Variables|Default|SetisOverlap true)
      (bind _outactors (Actor|GetAllActorsOfClass "/Game/Blueprints/BP_AutomaticDoorLever.BP_AutomaticDoorLever_C"))
      (for _array_element _outactors
        (bind _asbp_automatic_door_lever (Utilities|Casting|CastToBP_AutomaticDoorLever _array_element)
          (:then
            (Variables|Default|SetisSwitchOn (Variables|Default|GetisSwitchOn)))
          (:CastFailed
            (Development|PrintString "Cast Failed!" true false "(R=1.000000,G=0.000000,B=0.000000,A=1.000000)"))))
      (if (Variables|Default|GetisSwitchOn)
        (Variables|Default|SetisOpen true)
        ;[1 1 1] ドア開閉アニメーション処理
        (bind _slidedoor (Timeline|OpenDoor Play)
          (:Update
            (Transformation|SetRelativeLocation (Variables|Default|GetRightDoor) (Math|Vector|MakeVector 0.0 (+ _slidedoor (Variables|Default|GetrightDoorStartPosY)) 0.0) false false)
            (Transformation|SetRelativeLocation (Variables|Default|GetLeftDoor) (Math|Vector|MakeVector 0.0 (+ (Variables|Default|GetleftDoorStartPosY) (* _slidedoor -1.0)) 0.0) false false))
          (:Finished
            (Variables|Default|SetopenTimeCount 0.0)))
        (else
          (Variables|Default|SetisSwitchOn true))))))

(event OnComponentEndOverlap(m_pEventTriggerBox)
  (params (OverlappedComponent :type Primitive%20Component%20Object%20Reference) (OtherActor :type Actor%20Object%20Reference) (OtherComp :type Primitive%20Component%20Object%20Reference) (OtherBodyIndex :type Integer))
  ;[1 1 1] プレイヤーが検知外へいったら検知フラグを下げる
  (Variables|Default|SetisOverlap (not (Actor|ActorHasTag OtherActor "Player"))))

(event EventBeginPlay
  ;[1 1 1] 初期化(ドアの初期位置取得)
  (Variables|Default|SetrightDoorStartPosY (.y (.location (Transformation|GetRelativeTransform (Variables|Default|GetRightDoor)))))
  (Variables|Default|SetleftDoorStartPosY (.y (.location (Transformation|GetRelativeTransform (Variables|Default|GetLeftDoor))))))

(event EventTick
  (params (DeltaSeconds :type Float%20%28single-precision%29))
  ;[1 1 1] 開ききった時の処理(3秒毎にチェック)
  (if (Variables|Default|GetisOpen)
    (bind _output_get (Variables|Default|SetopenTimeCount (+ (Variables|Default|GetopenTimeCount) DeltaSeconds)))
    (if (not (< _output_get 3.0))
      (if (Variables|Default|GetisOverlap)
        (Variables|Default|SetopenTimeCount 0.0)
        (else
          (Variables|Default|SetisOpen false)
          (Variables|Default|SetopenTimeCount 0.0)
          ;[1 1 1] ドア開閉アニメーション処理
          (bind _slidedoor (Timeline|OpenDoor Reverse)
            (:Update
              (Transformation|SetRelativeLocation (Variables|Default|GetRightDoor) (Math|Vector|MakeVector 0.0 (+ _slidedoor (Variables|Default|GetrightDoorStartPosY)) 0.0) false false)
              (Transformation|SetRelativeLocation (Variables|Default|GetLeftDoor) (Math|Vector|MakeVector 0.0 (+ (Variables|Default|GetleftDoorStartPosY) (* _slidedoor -1.0)) 0.0) false false))
            (:Finished
              (Variables|Default|SetopenTimeCount 0.0))))))))

(fn ConstructionScript)

(fn IsMissionClear
  ;[1 1 1] ミッションが全て完成しているかを判定
  (bind _values (Utilities|Map|Values (Variables|Default|GetmissionMap)))
  (if (Utilities|Array|ContainsItem _values false)
    (Development|PrintString "Mission Unclear")
    (return false)
    (else
      (Development|PrintString "Mission Clear")
      (return true))))