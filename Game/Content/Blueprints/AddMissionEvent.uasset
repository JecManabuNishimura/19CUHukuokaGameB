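; AddMissionEvent is a trigger volume that updates the player's mission when they walk into it, using the MissionID it holds.
; On Box overlap it checks for the Player tag, casts to BP_PlayerCharacter and calls UpdateTheMission with update mode 0.
; It destroys itself after a short delay.
; An unconnected branch that would update BP_VRSmartPhone directly never runs.
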(event OnComponentBeginOverlap(Box)
  (params (OverlappedComponent :type Primitive%20Component%20Object%20Reference) (OtherActor :type Actor%20Object%20Reference) (OtherComp :type Primitive%20Component%20Object%20Reference) (OtherBodyIndex :type Integer) (bFromSweep :type Boolean) (SweepResult :type Hit%20Result%20Structure%20%28by%20ref%29))
  (if (Actor|ActorHasTag OtherActor "Player")
    (bind _asbp_player_character (Utilities|Casting|CastToBP_PlayerCharacter OtherActor))
    (Class|PlayerCharacter|UpdatetheMission _asbp_player_character 0 (Variables|Default|GetmissionID))
    (Utilities|FlowControl|Delay 0.2)
    (Actor|DestroyActor)))

(event EventBeginPlay)

(event Collision|EventActorBeginOverlap
  (params (OtherActor :type Actor%20Object%20Reference)))

(event EventTick
  (params (DeltaSeconds :type Float%20%28single-precision%29)))

(fn ConstructionScript)