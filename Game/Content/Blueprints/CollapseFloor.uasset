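; CollapseFloor is a trap floor actor that gives way under the player and reports the collapse to BP_TutorialGameMode.
; Overlapping Box with a Player-tagged actor disables player input, plays the collapse sound, turns off the Cube's collision and calls FloorCollapse on the game mode.
; A second trigger, Box1, plays its own floor-collapse sound only once through a DoOnce.
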(event OnComponentBeginOverlap(Box)
  (params (OverlappedComponent :type Primitive%20Component%20Object%20Reference) (OtherActor :type Actor%20Object%20Reference) (OtherComp :type Primitive%20Component%20Object%20Reference) (OtherBodyIndex :type Integer) (bFromSweep :type Boolean) (SweepResult :type Hit%20Result%20Structure%20%28by%20ref%29))
  (if (Actor|ActorHasTag OtherActor "Player")
    (Input|DisableInput (Game|GetPlayerController 0))
    (Audio|PlaySoundatLocation "/Game/SE/FloorCollapse.FloorCollapse" (Transformation|GetActorLocation) "0, 0, 0" 1.0 1.0 0.0 0 0 0)
    (Collision|SetCollisionEnabled (Variables|Default|GetCube) "NoCollision")
    (bind _asbp_tutorial_game_mode (Utilities|Casting|CastToBP_TutorialGameMode (Game|GetGameMode)))
    (Default|FloorCollapse _asbp_tutorial_game_mode)))

(event OnComponentBeginOverlap(Box1)
  (params (OverlappedComponent :type Primitive%20Component%20Object%20Reference) (OtherActor :type Actor%20Object%20Reference) (OtherComp :type Primitive%20Component%20Object%20Reference) (OtherBodyIndex :type Integer) (bFromSweep :type Boolean) (SweepResult :type Hit%20Result%20Structure%20%28by%20ref%29))
  (if (Actor|ActorHasTag OtherActor "Player")
    (Utilities|FlowControl|DoOnce false
      (:Completed
        (Audio|PlaySoundatLocation "/Game/SE/FloorCollapse_.FloorCollapse_" (Transformation|GetActorLocation) "0, 0, 0" 1.0 1.0 0.0 0 0 0)))))

(event EventBeginPlay)

(event Collision|EventActorBeginOverlap
  (params (OtherActor :type Actor%20Object%20Reference)))

(event EventTick
  (params (DeltaSeconds :type Float%20%28single-precision%29)))

(fn ConstructionScript)