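; Title screen pawn that places the player at the start position and shows either the VR or flat-screen title presentation.
; On BeginPlay it copies the location and rotation of a PlayerInitialPosActor marker, then destroys that marker.
; With an HMD enabled it unhides the BP_VR_TitleActor in the level; otherwise it adds a TitleWidget to the viewport.
; Both presentations appear only when the marker actor is found.
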(event EventBeginPlay
  ;[1 1 1] プレイヤーの初期位置設定(PlayerInitialPosActorの座標、回転情報をPlayerCharacterに渡す)
  (bind _returnvalue (Actor|GetActorOfClass "/Game/Blueprints/PlayerInitialPosActor.PlayerInitialPosActor_C"))
  (Utilities|IsValid _returnvalue
    (:Is%20Valid
      (Transformation|SetActorTransform (Math|Transform|MakeTransform (.location (Transformation|GetActorTransform _returnvalue)) (.rotation (Transformation|GetActorTransform _returnvalue)) "1,1,1"))
      (Actor|DestroyActor _returnvalue)
      (if (Class|HeadMountedDisplayFunctionLibrary|IsHeadMountedDisplayEnabled)
        (bind _returnvalue_2 (Actor|GetActorOfClass "/Game/Blueprints/BP_VR_TitleActor.BP_VR_TitleActor_C"))
        (Utilities|IsValid _returnvalue_2
          (:Is%20Valid
            (Rendering|SetActorHiddenInGame _returnvalue_2 false)))
        (else
          (bind _returnvalue_3 (UserInterface|CreateWidget "/Game/UI/TitleWidget.TitleWidget_C"))
          (bind _output_get (Variables|Default|SetTitleWidget _returnvalue_3))
          (UserInterface|Viewport|AddtoViewport _output_get 0))))))

(event Collision|EventActorBeginOverlap
  (params (OtherActor :type Actor%20Object%20Reference)))

(event EventTick
  (params (DeltaSeconds :type Float%20%28single-precision%29)))

(fn ConstructionScript)