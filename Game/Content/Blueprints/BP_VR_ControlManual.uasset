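; BP_VR_ControlManual is a temporary actor that displays a UI widget, apparently a control manual for VR.
; ChangeWidget creates a widget of the given class on the VRUI component and sets the display lifetime.
; Tick accumulates elapsed time and destroys the actor once it exceeds that lifetime.
; A player-reference check and an unused look-at-camera calculation are present, but neither feeds the shown event logic.
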(event Custom|ChangeWidget
  (params (Widget :type User%20Widget%20Class%20Reference) (MaxLifeTime :type Float%20%28single-precision%29))
  ;[1 1 1] Change Widget
  (bind _returnvalue (UserInterface|CreateWidget Widget))
  (UserInterface|SetWidget (Variables|Default|GetVR_UI) _returnvalue)
  (Variables|Default|SetDiappearTime MaxLifeTime))

(event EventBeginPlay)

(event EventTick
  (params (DeltaSeconds :type Float%20%28single-precision%29))
  ;[1 1 1] Destroy its self after X sec
  (Variables|Default|SetTime (+ DeltaSeconds (Variables|Default|GetTime)))
  (if (> (Variables|Default|GetTime) (Variables|Default|GetDiappearTime))
    (Actor|DestroyActor)))

(fn ConstructionScript)

(fn CheckPlayerRef
  (bind _returnvalue (Game|GetPlayerCharacter 0))
  (if (Utilities|IsValid (Variables|Default|GetPlayer1))
    (return)
    (elif (Utilities|IsValid _returnvalue)
      (bind _asbp_player_character (Utilities|Casting|CastToBP_PlayerCharacter _returnvalue)
        (:then
          (Variables|Default|SetPlayer1 _asbp_player_character)
          (if (Utilities|IsValid (Variables|Default|GetPlayer1))
            (return)
            (else
              (Development|PrintString "Failed To Acess  BP_PlayerCharacter" true true "(R=1.000000,G=0.000000,B=0.109215,A=1.000000)" 5.0))))
        (:CastFailed
          (Development|PrintString "Cast Failed of BP_PlayerCharacter" true true "(R=1.000000,G=0.000000,B=0.109215,A=1.000000)" 5.0)))
      (else
        (Development|PrintString "Can't Get Player in VRSmartPhone" true true "(R=1.000000,G=0.000000,B=0.109215,A=1.000000)" 5.0)))))