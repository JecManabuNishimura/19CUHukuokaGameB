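; VR smartphone actor that works as a photo camera and flashlight, with input enabled for player 0.
; Z or GrabRight draws the live display material into a photo render target, shows that photo on the screen for a set delay, then restores the live view.
; X toggles two camera light components.
; Photo export to disk, pixel readback and motion-controller attachment remain as unused, unconnected experiments.
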(event EventBeginPlay
  (Input|EnableInput (Game|GetPlayerController 0))
  (bind _outactors (Actor|GetAllActorsOfClass "/Script/hukuokaGame.PlayerCharacter"))
  (for (_array_element _array_index) _outactors
    (if (not (Math|Conversions|ToBoolean(Integer) _array_index))
      (Variables|Default|Setplayer1 _array_element))))

(event Collision|EventActorBeginOverlap
  (params (OtherActor :type Actor%20Object%20Reference)))

(event EventTick
  (params (DeltaSeconds :type Float%20%28single-precision%29)))

(event Input|ActionEvents|InputActionGrabRight
  (params (Key :type Key%20Structure :default "None"))
  ;[1 1 1] Change VR Smart Phone's display's material  when  took a photo.  It will display [Photo_ShowOutTime] seconds and change back to live mode.
  (:Pressed
    (if true
      (if (Variables|/Script/hukuokaGame.PlayerCharacter|Getvr_InCameraMode (Variables|Default|Getplayer1))
        _
        (else
          _))
      (Rendering|ClearRenderTarget2D "/Game/Materials/photoTarget.photoTarget" "(R=0.000000,G=0.000000,B=0.000000,A=255.000000)")
      (Rendering|DrawMaterialtoRenderTarget "/Game/Materials/photoTarget.photoTarget" "/Game/Materials/smartPhoneDisplay.SmartPhoneDisplay")
      (Rendering|Material|SetMaterial (Variables|Default|GetVRSmartPhoneDisplay) 0 "/Game/Materials/PhotoDisplay.PhotoDisplay")
      (Utilities|FlowControl|Delay (Variables|Default|GetPhoto_ShowOutTime))
      (Rendering|Material|SetMaterial (Variables|Default|GetVRSmartPhoneDisplay) 0 "/Game/Materials/smartPhoneDisplay.SmartPhoneDisplay"))))

(event Input|KeyboardEvents|C
  (params (Key :type Key%20Structure :default "None"))
  ;[1 1 1] [Not using] Save the photo to img_path (need to rotate if want to use)
)

(event Input|KeyboardEvents|Z
  (params (Key :type Key%20Structure :default "None"))
  ;[1 1 1] Change VR Smart Phone's display's material  when  took a photo.  It will display [Photo_ShowOutTime] seconds and change back to live mode.
  (:Pressed
    (if (Variables|/Script/hukuokaGame.PlayerCharacter|Getvr_InCameraMode (Variables|Default|Getplayer1))
      _
      (else
        _))
    (Rendering|ClearRenderTarget2D "/Game/Materials/photoTarget.photoTarget" "(R=0.000000,G=0.000000,B=0.000000,A=255.000000)")
    (Rendering|DrawMaterialtoRenderTarget "/Game/Materials/photoTarget.photoTarget" "/Game/Materials/smartPhoneDisplay.SmartPhoneDisplay")
    (Rendering|Material|SetMaterial (Variables|Default|GetVRSmartPhoneDisplay) 0 "/Game/Materials/PhotoDisplay.PhotoDisplay")
    (Utilities|FlowControl|Delay (Variables|Default|GetPhoto_ShowOutTime))
    (Rendering|Material|SetMaterial (Variables|Default|GetVRSmartPhoneDisplay) 0 "/Game/Materials/smartPhoneDisplay.SmartPhoneDisplay")))

(event Input|KeyboardEvents|X
  (params (Key :type Key%20Structure :default "None"))
  ;[1 1 1] VRのスマホライトOn/Off  / Change VR Smart Phone Camera Light on/off
  (:Pressed
    (if (Variables|Default|GetCameraLightOn)
      (Rendering|SetVisibility (Variables|Default|GetCameraLight) false false)
      (Rendering|SetVisibility (Variables|Default|GetCameraLight2) false false)
      (Variables|Default|SetCameraLightOn false)
      (else
        (Rendering|SetVisibility (Variables|Default|GetCameraLight) true false)
        (Rendering|SetVisibility (Variables|Default|GetCameraLight2) true false)
        (Variables|Default|SetCameraLightOn true)))))

(fn ConstructionScript)