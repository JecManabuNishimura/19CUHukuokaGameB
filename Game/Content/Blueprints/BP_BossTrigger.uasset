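; BP_BossTrigger is an overlap trigger that starts a boss encounter when the player enters with the linked lever switched on.
; It spawns a BP_AI_Enemy at the Spawner component, with glass-break and enemy voice sounds.
; It then flags the referenced Boss as a boss and enables its behavior; that reference is the spawn's Owner, not its result.
; The IsSpawn guard is checked but never set here.
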(event EventBeginPlay)

(event Collision|EventActorBeginOverlap
  (params (OtherActor :type Actor%20Object%20Reference))
  (bind _spawner (Variables|Default|GetSpawner))
  (bind _boss (Variables|Default|GetBoss))
  (bind _returnvalue (Transformation|GetWorldLocation _spawner))
  (if (not (Variables|Default|GetisSpawn))
    (if (Actor|ActorHasTag OtherActor "Player")
      (bind _asautomatic_door_lever (Utilities|Casting|CastToAutomaticDoorLever (Variables|Default|GetLever)))
      (if (Class|AutomaticDoorLever|GetLeverState _asautomatic_door_lever)
        (Game|SpawnActorfromClass "/Game/Blueprints/BP_AI_Enemy.BP_AI_Enemy_C" (Math|Transform|MakeTransform _returnvalue "0, 0, 0" (Transformation|GetWorldScale _spawner)) "Undefined" _boss 1.0 0)
        (Audio|PlaySoundatLocation "/Game/SE/Glass_Break.Glass_Break" _returnvalue "0, 0, 0" 1.0 1.0 0.0 0 0 0)
        (Audio|PlaySoundatLocation "/Game/SE/EnemyVoice.EnemyVoice" _returnvalue "0, 0, 0" 1.0 1.0 0.0 0 0 0)
        (bind _asbp_ai_enemy (Utilities|Casting|CastToBP_AI_Enemy _boss))
        (Variables|/Game/Blueprints/BP_AI_Enemy.BP_AI_Enemy_C|SetisBoss _asbp_ai_enemy true)
        (Default|SetCanRunBehavior _asbp_ai_enemy true)))))

(event EventTick
  (params (DeltaSeconds :type Float%20%28single-precision%29)))

(fn ConstructionScript)