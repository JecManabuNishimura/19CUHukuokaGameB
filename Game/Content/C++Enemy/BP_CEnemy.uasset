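; BP_CEnemy is an enemy Blueprint that reacts to noises made by the player through its pawn sensing component.
; When a noise instigator tagged Player is heard outside the two chase states and the attack state, it stores the player's location as the hear position and switches to the hear state.
; Other event stubs are empty, and an unconnected check against the hear state never runs.
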(event OnHearNoise(ppawnsensing_)
  (params (Instigator :type Pawn%20Object%20Reference) (Location :type Vector%20%28by%20ref%29 :default "0, 0, 0") (Volume :type Float%20%28single-precision%29))
  (if (Actor|ActorHasTag Instigator "Player")
    (if (Math|Boolean|ANDBoolean (Utilities|Enum|NotEqual(Enum) "kChase1" (Variables|Default|Getenemy_state_)) (Utilities|Enum|NotEqual(Enum) "kChase2" (Variables|Default|Getenemy_state_)) (Utilities|Enum|NotEqual(Enum) "kAttack" (Variables|Default|Getenemy_state_)))
      (bind _asbp_player_character (Utilities|Casting|CastToBP_PlayerCharacter Instigator))
      (Class|Enemy|SetHearPos (Transformation|GetActorLocation _asbp_player_character))
      (Class|Enemy|SetState "kHear"))))

(event EventBeginPlay)

(event Collision|EventActorBeginOverlap
  (params (OtherActor :type Actor%20Object%20Reference)))

(event EventTick
  (params (DeltaSeconds :type Float%20%28single-precision%29)))

(fn ConstructionScript)