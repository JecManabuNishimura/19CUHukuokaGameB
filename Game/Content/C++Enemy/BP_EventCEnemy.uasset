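; BP_EventCEnemy is a scripted event enemy that runs a route of target points once triggered, then destroys itself.
; While Trigger is set, Tick switches an idle enemy to KChase1 and plays its voice sound.
; In KChase2 it uses SimpleMoveToLocation toward the current point, advancing the index within a distance tolerance.
; The transition from KChase1 to KChase2 happens outside this graph.
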(event EventBeginPlay)

(event Collision|EventActorBeginOverlap
  (params (OtherActor :type Actor%20Object%20Reference)))

(event EventTick
  (params (DeltaSeconds :type Float%20%28single-precision%29))
  (bind _targetpoint_pos_ (Variables|Default|Gettargetpoint_pos_))
  (bind _targetpoint_pos__2 (Variables|Default|Gettargetpoint_pos_))
  (bind _tpindex (Variables|Default|GettpIndex))
  (bind _returnvalue (Utilities|Array|Length _targetpoint_pos_))
  (bind _output (Utilities|Array|Get(acopy) _targetpoint_pos__2 _tpindex))
  (if (Variables|Default|Gettrigger)
    (if (Utilities|Enum|Equal(Enum) (Variables|Default|Getenemy_state_) "kChase2")
      (if (== (Variables|Default|GettpIndex) _returnvalue)
        (Actor|DestroyActor)
        (else
          (AI|Navigation|SimpleMovetoLocation (Pawn|GetController self) _output)
          (if (Math|Vector|Equal(Vector) _output (Transformation|GetActorLocation) 5e+02)
            (if (not (== (Variables|Default|GettpIndex) _returnvalue))
              (Math|Integer|IncrementInt (Variables|Default|GettpIndex))))))
      (elif (Utilities|Enum|Equal(Enum) (Variables|Default|Getenemy_state_) "kIdle")
        (Class|Enemy|SetState "kChase1")
        (Audio|PlaySoundatLocation "/Game/SE/EnemyVoice.EnemyVoice" (Transformation|GetActorLocation) "0, 0, 0" 1.0 1.0 0.0 0 0 0)))))

(fn ConstructionScript)